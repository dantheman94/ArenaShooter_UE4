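; Arena character Blueprint that adds first-person arm animation for dashing and aiming down sights, plus a world-space health bar.
; BeginPlay binds dash, ADS and damage events and hands itself to the health bar widget.
; Timelines lerp the arms toward per-direction dash targets and back after a delay, or between the primary weapon's hip and ADS origins over its fire mode's aim time.
; The damage handler only casts the health bar widget.
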(event `self.ReceiveBeginPlay`
  (`|ExecutionSequence`
    (:`then_0`
      (`self.BindEvent_fDashAnimationEvent`)
      (`self.BindEvent_fAdsAnimationEvent`)
      (`self.BindEvent_fOnTakeDamage`))
    (:`then_1`
      (bind _asw_world_space_health_bar (cast `/Game/UMG/Ingame/HUD/Multiplayer/w_WorldSpaceHealthBar` (`WidgetComponent.GetUserWidgetObject` (`self.WorldSpaceHealthBar`))))
      (set `/Game/UMG/Ingame/HUD/Multiplayer/w_WorldSpaceHealthBar.Character` self _asw_world_space_health_bar))))

(event `BindEvent_fDashAnimationEvent`
  (add `self._fDashAnimationEvent` (delegate `DashFP_PlaceholderAnimationEvent`)))

(event `DashFP_PlaceholderAnimationEvent` :!signature `self._fDashAnimationEvent`
  (params (Direction :type "E_Direction Enum" :default "eGA_Fwd"))
  (bind _returnvalue (`KismetMathLibrary.Conv_ByteToInt` Direction))
  (bind _dashfpanimationexitduration (`self.DashFPAnimationExitDuration`))
  (bind _dashfpanimationenterduration (`self.DashFPAnimationEnterDuration`))
  (bind (_direction _timecurvee) (`Timeline|T_DashAnimationEnter` :!via `PlayFromStart` :!label _label)
    (:`Update`
      (if (< _timecurvee _dashfpanimationenterduration)
        (`SceneComponent.K2_SetRelativeTransform` (`self._FirstPerson_Arms`) (`KismetMathLibrary.TLerp` (`self._tFpArmsRelativeStarting`) (`|GetArrayItem` (`self.DashAnimationLerpTargets`) _returnvalue) (/ _timecurvee _dashfpanimationenterduration)) false false)
        (else
          (`|ExecutionSequence`
            (:`then_0`
              (goto _label :!via `Stop`))
            (:`then_1`
              (`KismetSystemLibrary.Delay` (`self.DashFPAnimationExitDelay`))
              (bind (_direction_2 _timecurvee_2) (`Timeline|T_DashAnimationExit` :!via `PlayFromStart` :!label _label_2)
                (:`Update`
                  (if (< _timecurvee_2 _dashfpanimationexitduration)
                    (`SceneComponent.K2_SetRelativeTransform` (`self._FirstPerson_Arms`) (`KismetMathLibrary.TLerp` (`|GetArrayItem` (`self.DashAnimationLerpTargets`) _returnvalue) (`self._tFpArmsRelativeStarting`) (/ _timecurvee_2 _dashfpanimationexitduration)) false false)
                    (else
                      (goto _label_2 :!via `Stop`))))))))))))

(event `BindEvent_fAdsAnimationEvent`
  (add `self._fAdsAnimationEvent` (delegate `Ads_PlaceholderAnimationEvent`)))

(event `Ads_PlaceholderAnimationEvent` :!signature `self._fAdsAnimationEvent`
  (params (AimingEnter :type Boolean))
  (bind _returnvalue (`self.GetPointerPrimaryWeapon`))
  (bind _returnvalue_2 (`self.GetPointerPrimaryWeapon`))
  (bind _returnvalue_3 (`Weapon.GetCurrentFireMode` _returnvalue_2))
  (bind _returnvalue_4 (`Weapon.GetCurrentFireMode` _returnvalue))
  (bind _returnvalue_5 (`Weapon.GetOriginHands` _returnvalue))
  (bind _returnvalue_6 (`FireMode.GetWeaponAimTime` _returnvalue_3))
  (bind _returnvalue_7 (`FireMode.GetOriginADS` _returnvalue_3))
  (bind _returnvalue_8 (`FireMode.GetWeaponAimTime` _returnvalue_4))
  (if (and AimingEnter (`FireMode.IsAimDownSightEnabled` (`Weapon.GetCurrentFireMode` (`self.GetPointerPrimaryWeapon`))))
    (bind (_direction _currenttime) (`Timeline|T_AdsOrigin_Enter` :!via `PlayFromStart` :!label _label_3)
      (:`Update`
        (if (<= _currenttime _returnvalue_6)
          (`self.UpdateOriginArmsTransform` (`KismetMathLibrary.TLerp` (`Weapon.GetOriginHands` _returnvalue_2) _returnvalue_7 (`KismetMathLibrary.NormalizeToRange` (/ _currenttime _returnvalue_6) 0.0 1.0) "EulerInterp"))
          (else
            (`self.UpdateOriginArmsTransform` _returnvalue_7)
            (goto _label_3 :!via `Stop`)))))
    (else
      (bind (_direction_2 _currenttime_2) (`Timeline|T_AdsOrigin_Exit` :!via `PlayFromStart` :!label _label_4)
        (:`Update`
          (if (<= _currenttime_2 _returnvalue_8)
            (`self.UpdateOriginArmsTransform` (`KismetMathLibrary.TLerp` (`FireMode.GetOriginADS` _returnvalue_4) _returnvalue_5 (`KismetMathLibrary.NormalizeToRange` (/ _currenttime_2 _returnvalue_8) 0.0 1.0) "EulerInterp"))
            (else
              (`self.UpdateOriginArmsTransform` _returnvalue_5)
              (goto _label_4 :!via `Stop`))))))))

(event `BindEvent_fOnTakeDamage`
  (add `self._fOnTakeDamage` (delegate `event_OnTakeDamage`)))

(event `event_OnTakeDamage` :!signature `self._fOnTakeDamage`
  (params (DamageAmount :type "Float (double-precision)"))
  (cast `/Game/UMG/Ingame/HUD/Multiplayer/w_WorldSpaceHealthBar` (`WidgetComponent.GetUserWidgetObject` (`self.WorldSpaceHealthBar`))))

(fn `UserConstructionScript`)