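; In-game multiplayer game state that runs the match intro, from loading screen and title to player control.
; With opening cinematics enabled, it hides HUDs and fades around cinematic events before switching to first person; otherwise it switches almost immediately.
; The switch either opens a buy menu with locked input or shows HUDs and auto-completes the intro.
; Intro completion restores game input and HUD for players in PlayerArray and adds a match title.
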(event `self.ReceiveBeginPlay`
  (add `self.IntroSequenceComplete` (delegate `BindIntroSequenceComplete`))
  (if (`self._bPlayOpeningCinematic`)
    (bind _returnvalue (`|CreateWidget` "/Game/UMG/Ingame/Screens/w_LoadingPlayers.w_LoadingPlayers_C" (`GameplayStatics.GetPlayerController` 0)))
    (`UserWidget.AddToViewport` _returnvalue 0)
    (`KismetSystemLibrary.Delay` (`/Game/UMG/Ingame/Screens/w_LoadingPlayers.Delay` _returnvalue))
    (bind _returnvalue_2 (`|CreateWidget` "/Game/UMG/Ingame/Screens/w_IngameMatchTitle.w_IngameMatchTitle_C" (`GameplayStatics.GetPlayerController` 0)))
    (bind _output_get (set `self.MatchTitle` _returnvalue_2))
    (`UserWidget.AddToViewport` _output_get 0)
    (for _array_element (`self.PlayerArray`)
      (bind _asbase_player_state (cast `BasePlayerState` _array_element))
      (bind ((`_PlayerController` __playercontroller)) (break `PlayerInfo` (`BasePlayerState._PlayerInfo` _asbase_player_state)))
      (`/Engine/EditorBlueprintResources/StandardMacros.IsValid` __playercontroller
        (:`Is Valid`
          (bind _asbp_ingame_hud (cast `/Game/Blueprints/Game/Multiplayer/BP_IngameHUD` (`PlayerController.GetHUD` __playercontroller)))
          (`BaseHUD.SetDisplayHud` _asbp_ingame_hud false))))
    (for _array_element_2 (`self._tOpeningCinematics`)
      (`/Engine/EditorBlueprintResources/StandardMacros.IsValid` _array_element_2
        (:`Is Valid`
          (add `CameraCinematic._OnCinematicStart` _array_element_2 (delegate `OnCinematicStart`))
          (add `CameraCinematic._OnHeadZoomThreshold` _array_element_2 (delegate `OnHeadZoomThreshold`)))))
    (else
      (`KismetSystemLibrary.Delay` 0.0)
      (`self.SwitchToFirstPerson AllClients`))))

(event `BindIntroSequenceComplete`
  (`self.IntroSequenceCompleteEvent`))

(event `OnHeadZoomThreshold`
  ;[0 0 0] Fade Out
  (`/Engine/EditorBlueprintResources/StandardMacros.DoOnce` false
    (:`Completed`
      (bind _returnvalue (`|CreateWidget` "/Game/UMG/w_FadeScreen.w_FadeScreen_C" (`GameplayStatics.GetPlayerController` 0) 0.15 (struct) (struct :`R` 1.0 :`G` 1.0 :`B` 1.0 :`A` 1.0)))
      (`UserWidget.AddToViewport` _returnvalue 1)
      (`/Game/UMG/w_FadeScreen.StartFade` _returnvalue 0.0 true 0.0)
      (`KismetSystemLibrary.Delay` 0.15)
      (`self.SwitchToFirstPerson AllClients`))))

(event `OnCinematicStart`
  (bind _returnvalue (`|CreateWidget` "/Game/UMG/w_FadeScreen.w_FadeScreen_C" (`GameplayStatics.GetPlayerController` 0) 2.0 (struct :`A` 1.0)))
  (`UserWidget.AddToViewport` _returnvalue 1)
  (`/Game/UMG/w_FadeScreen.StartFade` _returnvalue (+ (`/Game/UMG/Ingame/Screens/w_LoadingPlayers.Delay` (stale `self.ReceiveBeginPlay` _returnvalue)) 1.0) true 1.0)
  (`KismetSystemLibrary.PrintString` "Hello"))

(event `SwitchToFirstPerson AllClients`
  (bind _localplayercontroller (`self.LocalPlayerController`))
  (bind _matchtitle (`self.MatchTitle`))
  (if (`self._bShowBuyMenu`)
    (bind _returnvalue (`|CreateWidget` "/Game/UMG/Ingame/Screens/BuyMenu/w_BuyMenu_V2.w_BuyMenu_V2_C" (`GameplayStatics.GetPlayerController` 0)))
    (`UserWidget.AddToViewport` _returnvalue 0)
    (for _array_element (`self.PlayerArray`)
      (bind _asbase_player_state (cast `BasePlayerState` _array_element))
      (bind ((`_PlayerController` __playercontroller)) (break `PlayerInfo` (`BasePlayerState._PlayerInfo` _asbase_player_state)))
      (`/Engine/EditorBlueprintResources/StandardMacros.IsValid` __playercontroller
        (:`Is Valid`
          (bind _output_get (set `self.LocalPlayerController` __playercontroller))
          (set `PlayerController.bShowMouseCursor` true _output_get)
          (`WidgetBlueprintLibrary.SetInputMode_UIOnlyEx` _output_get _returnvalue "LockAlways")
          (`Controller.SetIgnoreLookInput` _output_get true)
          (`Controller.SetIgnoreMoveInput` _output_get true)
          (`/Engine/EditorBlueprintResources/StandardMacros.IsValid` _matchtitle :!label _label
            (:`Is Valid`
              (`Widget.RemoveFromParent` _matchtitle))
            (:`Is Not Valid`
              _))
          (`PlayerController.SetViewTargetWithBlend` _localplayercontroller (`Controller.K2_GetPawn` _localplayercontroller) 0.0 "VTBlend_Linear" 0.0 false)
          (bind _returnvalue_2 (`|CreateWidget` "/Game/UMG/w_FadeScreen.w_FadeScreen_C" null 0.5 (struct :`R` 1.0 :`G` 1.0 :`B` 1.0 :`A` 1.0)))
          (`UserWidget.AddToViewport` _returnvalue_2 1)
          (`/Game/UMG/w_FadeScreen.StartFade` _returnvalue_2 0.15 true 1.0))))
    (else
      ;[0 0 0] Show Hud
      (for _array_element_2 (`self.PlayerArray`)
        (bind _asbase_player_state_2 (cast `BasePlayerState` _array_element_2))
        (bind ((`_PlayerController` __playercontroller_2)) (break `PlayerInfo` (`BasePlayerState._PlayerInfo` _asbase_player_state_2)))
        (`/Engine/EditorBlueprintResources/StandardMacros.IsValid` __playercontroller_2
          (:`Is Valid`
            (bind _output_get_2 (set `self.LocalPlayerController` __playercontroller_2))
            (bind _asbp_ingame_hud (cast `/Game/Blueprints/Game/Multiplayer/BP_IngameHUD` (`PlayerController.GetHUD` _output_get_2)))
            (`BaseHUD.SetDisplayHud` _asbp_ingame_hud true)
            (`|ExecutionSequence`
              (:`then_0`
                (goto _label))
              (:`then_1`
                (`KismetSystemLibrary.Delay` 1.0)
                (`self.IntroSequenceCompleteEvent`)))))))))

(event `IntroSequenceCompleteEvent`
  (for _array_element (`self.PlayerArray`)
    (bind _asbase_player_state (cast `BasePlayerState` _array_element))
    (bind ((`_PlayerController` __playercontroller)) (break `PlayerInfo` (`BasePlayerState._PlayerInfo` _asbase_player_state)))
    (`/Engine/EditorBlueprintResources/StandardMacros.IsValid` __playercontroller
      (:`Is Valid`
        (bind _output_get (set `self.LocalPlayerController` __playercontroller))
        (set `PlayerController.bShowMouseCursor` false _output_get)
        (`WidgetBlueprintLibrary.SetInputMode_GameOnly` _output_get)
        (`Controller.SetIgnoreLookInput` _output_get false)
        (`Controller.SetIgnoreMoveInput` _output_get false)
        (bind _asbp_ingame_hud (cast `/Game/Blueprints/Game/Multiplayer/BP_IngameHUD` (`PlayerController.GetHUD` __playercontroller)))
        (`BaseHUD.SetDisplayHud` _asbp_ingame_hud true))))
  (bind _returnvalue (`|CreateWidget` "/Game/UMG/Ingame/HUD/Multiplayer/w_MatchTitle.w_MatchTitle_C" (`GameplayStatics.GetPlayerController` 0)))
  (`UserWidget.AddToViewport` _returnvalue 0)
  (`KismetSystemLibrary.PrintString` "Hello"))

(fn `UserConstructionScript`)