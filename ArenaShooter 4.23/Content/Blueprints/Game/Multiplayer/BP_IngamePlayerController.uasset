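; In-game player controller, in a multiplayer folder, that toggles the pause screen with Escape or F10.
; Tick polls both keys and drives a FlipFlop, which the Unpause event also triggers when its state check passes.
; The FlipFlop switches mouse cursor, input and BP_IngameHUD display while adding or removing a lazily created, reused W_PauseScreen.
; It does not pause the game simulation itself.
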(event `self.ReceiveTick`
  (params (DeltaSeconds :type "Float (single-precision)"))
  (`parent.ReceiveTick` DeltaSeconds)
  (`self.Tick_CheckForPause`))

(event `Unpause`
  (bind _w_pausescreen (`self.w_PauseScreen`))
  (if (stale _isa)
    (bind _isa (`/Engine/EditorBlueprintResources/StandardMacros.FlipFlop` :!label _label)
      (:`A`
        (set `self.bShowMouseCursor` true)
        (`self.DisableInput` self)
        (bind _asbp_ingame_hud (cast `/Game/Blueprints/Game/Multiplayer/BP_IngameHUD` (`self.GetHUD`)))
        (`BaseHUD.SetDisplayHud` _asbp_ingame_hud false)
        (`/Engine/EditorBlueprintResources/StandardMacros.IsValid` (`self.w_PauseScreen`)
          (:`Is Valid`
            _)
          (:`Is Not Valid`
            (bind _returnvalue (`|CreateWidget` "/Game/UMG/Ingame/Screens/w_PauseScreen.w_PauseScreen_C" self))
            (bind _output_get (set `self.w_PauseScreen` _returnvalue))))
        (if (not (`Widget.IsInViewport` _output_get))
          (`UserWidget.AddToViewport` (`self.w_PauseScreen`) 0)))
      (:`B`
        (set `self.bShowMouseCursor` false)
        (`self.EnableInput` self)
        (bind _asbp_ingame_hud_2 (cast `/Game/Blueprints/Game/Multiplayer/BP_IngameHUD` (`self.GetHUD`)))
        (`BaseHUD.SetDisplayHud` _asbp_ingame_hud_2 true)
        (`/Engine/EditorBlueprintResources/StandardMacros.IsValid` _w_pausescreen
          (:`Is Valid`
            (if (`Widget.IsInViewport` _w_pausescreen)
              (`Widget.RemoveFromParent` _w_pausescreen))))))))

(event `Tick_CheckForPause`
  (if (or (`self.WasInputKeyJustPressed` "Escape") (`self.WasInputKeyJustPressed` "F10"))
    (goto _label)))

(fn `UserConstructionScript`
  (`parent.UserConstructionScript`))