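; BP_SpawnVolume is a placeable spawn volume that serves the game types listed in its GameModes array.
; On BeginPlay it waits a zero-second Delay, then registers itself with the IngameGameMode for each listed entry matching the current game type.
; The construction script sets up graphics for gametype, team and spawn name text and sizes the SpawnBounds box from BoundsHalfExtents.
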(event `self.ReceiveBeginPlay`
  (`KismetSystemLibrary.Delay` 0.0)
  (for _array_element (`self._GameModes`)
    (bind _asingame_game_mode (cast `IngameGameMode` (`GameplayStatics.GetGameMode`)))
    (if (`|EnumEquality` (`IngameGameMode.GetGameType` _asingame_game_mode) _array_element)
      (`IngameGameMode.RegisterSpawnVolumeWithGametype` _asingame_game_mode self))))

(fn `UserConstructionScript`
  (`self.SetupGraphics` (`self._Text_Gamemode`) (`self._Text_Team`) (`self._Text_SpawnVolume`))
  (`BoxComponent.SetBoxExtent` (`self._SpawnBounds`) (`self._BoundsHalfExtents`) true))