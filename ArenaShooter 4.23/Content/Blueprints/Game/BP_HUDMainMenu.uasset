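; Main menu HUD that shows and hides the splash, main menu, loading, host/client lobby and roster widgets.
; Show events call their parent, lazily create and cache each widget from a class variable, then add it to the viewport, printing an error if the class is null.
; Lobby events choose screens by the Hosting flag.
; Showing the roster refreshes the GameState player list, and the loading screen receives a message.
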(event `HideAllMainMenus`
  (bind __ui_lobbyroster_instance (`self._UI_LobbyRoster_Instance`))
  (bind __ui_mainmenu_instance (`self._UI_MainMenu_Instance`))
  (bind __ui_hostlobby_instance (`self._UI_HostLobby_Instance`))
  (bind __ui_clientlobby_instance (`self._UI_ClientLobby_Instance`))
  (`|ExecutionSequence`
    (:`then_0`
      (`/Engine/EditorBlueprintResources/StandardMacros.IsValid` __ui_mainmenu_instance
        (:`Is Valid`
          (`Widget.RemoveFromParent` __ui_mainmenu_instance))))
    (:`then_1`
      (`/Engine/EditorBlueprintResources/StandardMacros.IsValid` __ui_hostlobby_instance
        (:`Is Valid`
          (`Widget.RemoveFromParent` __ui_hostlobby_instance))))
    (:`then_2`
      (`/Engine/EditorBlueprintResources/StandardMacros.IsValid` __ui_clientlobby_instance
        (:`Is Valid`
          (`Widget.RemoveFromParent` __ui_clientlobby_instance))))
    (:`then_3`
      (`/Engine/EditorBlueprintResources/StandardMacros.IsValid` __ui_lobbyroster_instance
        (:`Is Valid`
          (`Widget.RemoveFromParent` __ui_lobbyroster_instance))))))

(event `self.ShowUI_Splash`
  (`parent.ShowUI_Splash`)
  (`/Engine/EditorBlueprintResources/StandardMacros.IsValid` (`self._UI_SplashScreen_Instance`)
    (:`Is Valid`
      (if (not (`Widget.IsInViewport` (stale _output_get))) :!label _label
        (`UserWidget.AddToViewport` (`self._UI_SplashScreen_Instance`) 0)))
    (:`Is Not Valid`
      (if (`KismetSystemLibrary.IsValidClass` (`self._UI_SplashScreen_Class`))
        (bind _returnvalue (`|CreateWidget` (`self._UI_SplashScreen_Class`) (`self.GetOwningPlayerController`)))
        (bind _output_get (set `self._UI_SplashScreen_Instance` _returnvalue))
        (goto _label)
        (else
          (`KismetSystemLibrary.PrintString` "ERROR: _UI_SplashScreen_Class is NULL" true false (struct :`R` 1.0 :`A` 1.0) 5.0))))))

(event `self.ShowUI_LobbyRoster`
  (params (ZOrder :type Integer))
  (bind __ui_lobbyroster_instance (`self._UI_LobbyRoster_Instance`))
  (`parent.ShowUI_LobbyRoster` ZOrder)
  (`/Engine/EditorBlueprintResources/StandardMacros.IsValid` __ui_lobbyroster_instance
    (:`Is Valid`
      (`Widget.RemoveFromParent` __ui_lobbyroster_instance)
      (if (not (`Widget.IsInViewport` (stale _output_get))) :!label _label_2
        (`UserWidget.AddToViewport` (`self._UI_LobbyRoster_Instance`) ZOrder)
        (bind _asbase_game_state (cast `BaseGameState` (`GameplayStatics.GetGameState`)))
        (`BaseGameState.UpdatePlayerList` _asbase_game_state)))
    (:`Is Not Valid`
      (if (`KismetSystemLibrary.IsValidClass` (`self._UI_LobbyRoster_Class`))
        (bind _returnvalue (`|CreateWidget` (`self._UI_LobbyRoster_Class`) (`self.GetOwningPlayerController`)))
        (bind _output_get (set `self._UI_LobbyRoster_Instance` _returnvalue))
        (goto _label_2)
        (else
          (`KismetSystemLibrary.PrintString` "ERROR: _UI_LobbyRoster_Class is NULL" true false (struct :`R` 1.0 :`A` 1.0) 5.0))))))

(event `self.ShowUI_MainMenu`
  (params (ZOrder :type Integer))
  (`parent.ShowUI_MainMenu` ZOrder)
  (`/Engine/EditorBlueprintResources/StandardMacros.IsValid` (`self._UI_MainMenu_Instance`)
    (:`Is Valid`
      (if (not (`Widget.IsInViewport` (stale _output_get))) :!label _label_3
        (`UserWidget.AddToViewport` (`self._UI_MainMenu_Instance`) ZOrder)))
    (:`Is Not Valid`
      (if (`KismetSystemLibrary.IsValidClass` (`self._UI_MainMenu_Class`))
        (bind _returnvalue (`|CreateWidget` (`self._UI_MainMenu_Class`) (`self.GetOwningPlayerController`)))
        (bind _output_get (set `self._UI_MainMenu_Instance` _returnvalue))
        (goto _label_3)
        (else
          (`KismetSystemLibrary.PrintString` "ERROR: _UI_MainMenu_Class is NULL" true false (struct :`R` 1.0 :`A` 1.0) 5.0))))))

(event `self.ShowUI_LoadingServer`
  (params (Message :type "Text (by ref)") (ZOrder :type Integer))
  (bind __ui_loadingserver_instance (`self._UI_LoadingServer_Instance`))
  (`parent.ShowUI_LoadingServer` Message ZOrder)
  (`/Engine/EditorBlueprintResources/StandardMacros.IsValid` (`self._UI_LoadingServer_Instance`)
    (:`Is Valid`
      (if (not (`Widget.IsInViewport` (stale _output_get))) :!label _label_4
        (`UserWidget.AddToViewport` __ui_loadingserver_instance ZOrder)
        (bind _asw_loading_screen (cast `/Game/UMG/MainMenu/Local/w_LoadingScreen` __ui_loadingserver_instance))
        (set `/Game/UMG/MainMenu/Local/w_LoadingScreen.Text` Message _asw_loading_screen)))
    (:`Is Not Valid`
      (if (`KismetSystemLibrary.IsValidClass` (`self._UI_LoadingServer_Class`))
        (bind _returnvalue (`|CreateWidget` (`self._UI_LoadingServer_Class`) (`self.GetOwningPlayerController`)))
        (bind _output_get (set `self._UI_LoadingServer_Instance` _returnvalue))
        (goto _label_4)
        (else
          (`KismetSystemLibrary.PrintString` "ERROR: _UI_LoadingServer_Class is NULL" true false (struct :`R` 1.0 :`A` 1.0) 5.0))))))

(event `self.ShowUI_LobbyPrematch`
  (params (Hosting :type Boolean) (ZOrder :type Integer))
  (`parent.ShowUI_LobbyPrematch` Hosting ZOrder)
  (`self.HideUI_HostLobby`)
  (`self.HideUI_ClientLobby`)
  (if Hosting
    (`self.ShowUI_HostLobby` ZOrder)
    (else
      (`self.ShowUI_ClientLobby` ZOrder))))

(event `self.ShowUI_HostLobby`
  (params (ZOrder :type Integer))
  (bind __ui_hostlobby_instance (`self._UI_HostLobby_Instance`))
  (`parent.ShowUI_HostLobby` ZOrder)
  (`/Engine/EditorBlueprintResources/StandardMacros.IsValid` __ui_hostlobby_instance
    (:`Is Valid`
      (`Widget.RemoveFromParent` __ui_hostlobby_instance)
      (if (not (`Widget.IsInViewport` (stale _output_get))) :!label _label_5
        (`UserWidget.AddToViewport` (`self._UI_HostLobby_Instance`) ZOrder)))
    (:`Is Not Valid`
      (if (`KismetSystemLibrary.IsValidClass` (`self._UI_HostLobby_Class`))
        (bind _returnvalue (`|CreateWidget` (`self._UI_HostLobby_Class`) (`self.GetOwningPlayerController`)))
        (bind _output_get (set `self._UI_HostLobby_Instance` _returnvalue))
        (goto _label_5)
        (else
          (`KismetSystemLibrary.PrintString` "ERROR: _UI_HostLobby_Class is NULL" true false (struct :`R` 1.0 :`A` 1.0) 5.0))))))

(event `self.HideUI_HostLobby`
  (bind __ui_hostlobby_instance (`self._UI_HostLobby_Instance`))
  (`parent.HideUI_HostLobby`)
  (`/Engine/EditorBlueprintResources/StandardMacros.IsValid` __ui_hostlobby_instance
    (:`Is Valid`
      (`Widget.RemoveFromParent` __ui_hostlobby_instance))))

(event `self.ShowUI_LobbyMainMenu`
  (params (Hosting :type Boolean) (ZOrder :type Integer))
  (`parent.ShowUI_LobbyMainMenu` Hosting ZOrder)
  (`self.HideUI_MainMenu`)
  (`self.HideUI_ClientLobby`)
  (if Hosting
    (`self.ShowUI_MainMenu` ZOrder)
    (else
      (`self.ShowUI_ClientLobby` ZOrder))))

(event `self.ShowUI_ClientLobby`
  (params (ZOrder :type Integer))
  (bind __ui_clientlobby_instance (`self._UI_ClientLobby_Instance`))
  (`parent.ShowUI_ClientLobby` ZOrder)
  (`/Engine/EditorBlueprintResources/StandardMacros.IsValid` __ui_clientlobby_instance
    (:`Is Valid`
      (`Widget.RemoveFromParent` __ui_clientlobby_instance)
      (if (not (`Widget.IsInViewport` (stale _output_get))) :!label _label_6
        (`UserWidget.AddToViewport` (`self._UI_ClientLobby_Instance`) ZOrder)))
    (:`Is Not Valid`
      (if (`KismetSystemLibrary.IsValidClass` (`self._UI_ClientLobby_Class`))
        (bind _returnvalue (`|CreateWidget` (`self._UI_ClientLobby_Class`) (`self.GetOwningPlayerController`)))
        (bind _output_get (set `self._UI_ClientLobby_Instance` _returnvalue))
        (goto _label_6)
        (else
          (`KismetSystemLibrary.PrintString` "ERROR: _UI_ClientLobby_Class is NULL" true false (struct :`R` 1.0 :`A` 1.0) 5.0))))))

(event `self.HideUI_ClientLobby`
  (bind __ui_clientlobby_instance (`self._UI_ClientLobby_Instance`))
  (`parent.HideUI_ClientLobby`)
  (`/Engine/EditorBlueprintResources/StandardMacros.IsValid` __ui_clientlobby_instance
    (:`Is Valid`
      (`Widget.RemoveFromParent` __ui_clientlobby_instance))))

(fn `UserConstructionScript`)