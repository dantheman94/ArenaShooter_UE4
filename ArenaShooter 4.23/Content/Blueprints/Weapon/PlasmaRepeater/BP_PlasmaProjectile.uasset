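; Plasma Repeater projectile Blueprint that sets up the look of the shot's mesh and light.
; The construction script creates a dynamic instance of M_DefaultProjectile on the static mesh and feeds it the projectile colour and opacity variables.
; The same colour drives the point light, so the glow matches the mesh.
; The event graph adds no logic of its own, only passing BeginPlay to the parent class.
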(event `self.ReceiveBeginPlay`
  (`parent.ReceiveBeginPlay`))

(fn `UserConstructionScript`
  (bind _projectilecolour (`self.ProjectileColour`))
  (`parent.UserConstructionScript`)
  (bind _returnvalue (`PrimitiveComponent.CreateDynamicMaterialInstance` (`self._StaticMesh`) 0 "/Game/Materials/Weapons/M_DefaultProjectile.M_DefaultProjectile" "None"))
  (`MaterialInstanceDynamic.SetScalarParameterValue` _returnvalue "Opacity" (`self.ProjectileOpacity`))
  (`MaterialInstanceDynamic.SetVectorParameterValue` _returnvalue "BaseColour" _projectilecolour)
  (`LightComponent.SetLightColor` (`self.PointLight`) _projectilecolour true))