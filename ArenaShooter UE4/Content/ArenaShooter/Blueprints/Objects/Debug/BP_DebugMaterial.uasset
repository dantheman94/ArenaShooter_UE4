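; BP_DebugMaterial is a debug display actor for previewing a material and physical material on a small booth of floor, walls and sphere.
; The construction script applies the Material and Physics variables to each mesh as its slot 0 material and physical material override.
; A text render labels the booth with the material's display name.
; The event graph holds only disabled placeholder events, so there is no runtime logic.
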(fn `UserConstructionScript`
  (bind _material (`self.Material`))
  (`PrimitiveComponent.SetMaterial` (`self.floor`) 0 (`self.Material`))
  (`PrimitiveComponent.SetMaterial` (`self.wallback`) 0 (`self.Material`))
  (`PrimitiveComponent.SetMaterial` (`self.wallside1`) 0 (`self.Material`))
  (`PrimitiveComponent.SetMaterial` (`self.wallside2`) 0 (`self.Material`))
  (`PrimitiveComponent.SetMaterial` (`self.sphere`) 0 _material)
  (`TextRenderComponent.K2_SetText` (`self.TextRender`) (`KismetTextLibrary.Conv_StringToText` (`KismetSystemLibrary.GetDisplayName` _material)))
  (`PrimitiveComponent.SetPhysMaterialOverride` (`self.floor`) (`self.Physics`))
  (`PrimitiveComponent.SetPhysMaterialOverride` (`self.wallback`) (`self.Physics`))
  (`PrimitiveComponent.SetPhysMaterialOverride` (`self.wallside1`) (`self.Physics`))
  (`PrimitiveComponent.SetPhysMaterialOverride` (`self.wallside2`) (`self.Physics`))
  (`PrimitiveComponent.SetPhysMaterialOverride` (`self.sphere`) (`self.Physics`)))