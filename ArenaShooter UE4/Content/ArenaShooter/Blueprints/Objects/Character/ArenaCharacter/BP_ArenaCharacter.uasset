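; Arena shooter player character Blueprint with first-person arm motion, wall running and grapple hook logic.
; BeginPlay binds parent events, with timelines lerping the arm transform as placeholder dash and aim-down-sights animations.
; Wall running zeroes gravity and re-traces the wall to steer velocity along it.
; Grapple code uses sphere traces, a cable and curve-driven forces, but its throw entry, wall-run exit and sprint arm animation are disconnected.
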(event `self.ReceiveBeginPlay`
  (`|ExecutionSequence`
    (:`then_0`
      (`self.BindEvent_fDashAnimationEvent`)
      (`self.BindEvent_fAdsAnimationEvent`)
      (`self.BindEvent_fOnTakeDamage`)
      (`self.BindEvent_StartSprinting`))
    (:`then_1`
      (`MovementComponent.SetPlaneConstraintEnabled` (`self.CharacterMovement`) false)
      (`self.BindGrappleHook`))))

(event `self.ReceiveTick`
  (params (DeltaSeconds :type "Float (single-precision)")))

(event `BindEvent_fDashAnimationEvent`
  (add `self._fDashAnimationEvent` (delegate `DashFP_PlaceholderAnimationEvent`)))

(event `BindEvent_fAdsAnimationEvent`
  (add `self._fAdsAnimationEvent` (delegate `Ads_PlaceholderAnimationEvent`)))

(event `BindEvent_StartSprinting`
  (add `self._fOnSprintEnter` (delegate `event_OnStartSprinting`)))

(event `event_OnStartSprinting` :!signature `self._fOnSprintEnter`
  (params (IsSprinting :type Boolean)))

(event `DashFP_PlaceholderAnimationEvent` :!signature `self._fDashAnimationEvent`
  (params (Direction :type "E_Direction Enum" :default "eGA_Fwd"))
  (bind _returnvalue (`KismetMathLibrary.Conv_ByteToInt` Direction))
  (bind _dashfpanimationexitduration (`self.DashFPAnimationExitDuration`))
  (bind _dashfpanimationenterduration (`self.DashFPAnimationEnterDuration`))
  (bind (_direction _timecurvee) (`Timeline|T_DashAnimationEnter` :!via `PlayFromStart` :!label _label)
    (:`Update`
      (if (and (< _timecurvee _dashfpanimationenterduration) (not (`self.IsSliding`)))
        (`SceneComponent.K2_SetRelativeTransform` (`self._FirstPerson_Arms`) (`KismetMathLibrary.TLerp` (`self._tFpArmsRelativeStarting`) (`|GetArrayItem` (`self.DashAnimationLerpTargets`) _returnvalue) (/ _timecurvee _dashfpanimationenterduration)) false false)
        (else
          (`|ExecutionSequence`
            (:`then_0`
              (goto _label :!via `Stop`))
            (:`then_1`
              (`KismetSystemLibrary.Delay` (`self.DashFPAnimationExitDelay`))
              (bind (_direction_2 _timecurvee_2) (`Timeline|T_DashAnimationExit` :!via `PlayFromStart` :!label _label_2)
                (:`Update`
                  (if (and (not (`self.IsSliding`)) (< _timecurvee_2 _dashfpanimationexitduration))
                    (`SceneComponent.K2_SetRelativeTransform` (`self._FirstPerson_Arms`) (`KismetMathLibrary.TLerp` (`|GetArrayItem` (`self.DashAnimationLerpTargets`) _returnvalue) (`self._tFpArmsRelativeStarting`) (/ _timecurvee_2 _dashfpanimationexitduration)) false false)
                    (else
                      (goto _label_2 :!via `Stop`))))))))))))

(event `Ads_PlaceholderAnimationEvent` :!signature `self._fAdsAnimationEvent`
  (params (AimingEnter :type Boolean))
  (bind _returnvalue (`self.GetPointerPrimaryWeapon`))
  (bind _returnvalue_2 (`self.GetPointerPrimaryWeapon`))
  (bind _returnvalue_3 (`Weapon.GetCurrentFireMode` _returnvalue))
  (bind _returnvalue_4 (`Weapon.GetCurrentFireMode` _returnvalue_2))
  (bind _returnvalue_5 (`Weapon.GetOriginHands` _returnvalue_2))
  (bind _returnvalue_6 (`FireMode.GetWeaponAimTime` _returnvalue_3))
  (bind _returnvalue_7 (`FireMode.GetOriginADS` _returnvalue_3))
  (bind _returnvalue_8 (`FireMode.GetWeaponAimTime` _returnvalue_4))
  (if (and AimingEnter (`FireMode.IsAimDownSightEnabled` (`Weapon.GetCurrentFireMode` (`self.GetPointerPrimaryWeapon`))))
    (bind (_direction _currenttime) (`Timeline|T_AdsOrigin_Enter` :!via `PlayFromStart` :!label _label_3)
      (:`Update`
        (if (<= _currenttime _returnvalue_6)
          (`self.UpdateOriginArmsTransform` (`KismetMathLibrary.TLerp` (`Weapon.GetOriginHands` _returnvalue) _returnvalue_7 (`KismetMathLibrary.NormalizeToRange` (/ _currenttime _returnvalue_6) 0.0 1.0) "EulerInterp"))
          (else
            (`self.UpdateOriginArmsTransform` _returnvalue_7)
            (goto _label_3 :!via `Stop`)))))
    (else
      (bind (_direction_2 _currenttime_2) (`Timeline|T_AdsOrigin_Exit` :!via `PlayFromStart` :!label _label_4)
        (:`Update`
          (if (<= _currenttime_2 _returnvalue_8)
            (`self.UpdateOriginArmsTransform` (`KismetMathLibrary.TLerp` (`FireMode.GetOriginADS` _returnvalue_4) _returnvalue_5 (`KismetMathLibrary.NormalizeToRange` (/ _currenttime_2 _returnvalue_8) 0.0 1.0) "EulerInterp"))
            (else
              (`self.UpdateOriginArmsTransform` _returnvalue_5)
              (goto _label_4 :!via `Stop`))))))))

(event `BindEvent_fOnTakeDamage`
  (add `self._fOnTakeDamage` (delegate `event_OnTakeDamage`)))

(event `event_OnTakeDamage` :!signature `self._fOnTakeDamage`
  (params (DamageAmount :type "Float (double-precision)")))

(event `BeginWallRun`
  (bind _charactermovement (`self.CharacterMovement`))
  (set `CharacterMovementComponent.AirControl` 1.0 _charactermovement)
  (set `CharacterMovementComponent.GravityScale` 0.0 _charactermovement)
  (`MovementComponent.SetPlaneConstraintNormal` _charactermovement (0.0 0.0 1.0))
  (set `self.IsWallRunning_0` true)
  (`Timeline|T_UpdateWallRun`
    (:`Update`
      (`self.UpdateWallRun`))))

(event `BindGrappleHook`
  (add `self._fOnGrappleHook` (delegate `OnGrappleHook`))
  (add `self._fOnGrappleHookRelease` (delegate `OnGrappleHookRelease`)))

(event `OnGrappleHook`)

(event `OnGrappleHookRelease`
  (bind _charactermovement (`self.CharacterMovement`))
  (bind _grapplehookanchoractor (`self.GrappleHookAnchorActor`))
  (bind _bp_stamina_grapple (`self.BP_Stamina_Grapple`))
  (bind _grapplehookthrowduration (`self.GrappleHookThrowDuration`))
  (bind _grapplehookanchorpoint (`self.GrappleHookAnchorPoint`))
  (bind _grapplehookcable (`self.GrappleHookCable`))
  (bind _grapplehookanchorpoint_2 (`self.GrappleHookAnchorPoint`))
  (bind _grapplehookanchoractor_2 (`self.GrappleHookAnchorActor`))
  (bind _grapplestartinglocation (`self.GrappleStartingLocation`))
  (bind _grapplehookanchoractor_3 (`self.GrappleHookAnchorActor`))
  (bind _returnvalue (`SceneComponent.K2_GetComponentLocation` (`self.GrappleHookOrigin`)))
  (bind _returnvalue_2 (- (`self.K2_GetActorLocation`) (`self.GrappleHookAnchorPoint`)))
  (if (`self.GrappleConnected`)
    (set `self.GrappleConnected` false)
    (`PrimitiveComponent.SetCollisionEnabled` (`self.GrappleHookCable`) "NoCollision")
    (`/Engine/EditorBlueprintResources/StandardMacros.IsValid` _grapplehookanchoractor_2
      (:`Is Valid`
        (`self.K2_DestroyActor` _grapplehookanchoractor_2))
      (:`Is Not Valid`
        _))
    (`CableComponent.SetAttachEndTo` _grapplehookcable null "None" "None")
    (`PrimitiveComponent.SetSimulatePhysics` (`self.CapsuleComponent`) false)
    (`SceneComponent.SetVisibility` (`self.GrappleHookCable`) false false)
    (set `CharacterMovementComponent.AirControl` (`self._fDefaultAirControl`) (`self.CharacterMovement`))
    (`|ExecutionSequence`
      (:`then_0`
        (`Stamina.ClearStamina` _bp_stamina_grapple)
        (`Stamina.DelayedRecharge` _bp_stamina_grapple))
      (:`then_1`
        (bind (_direction _time) (`Timeline|T_GrappleHookSwing` :!via `Stop` :!label _label_5)
          (:`Update`
            (if (`self.GrappleConnected`)
              (bind _returnvalue_3 (/ _time (`self.GrappleHookSwingDuration`)))
              (`self.DebugMessage` (`KismetStringLibrary.Concat_StrStr` "Alpha: " (`KismetStringLibrary.Conv_DoubleToString` _returnvalue_3)) false)
              (if (< _returnvalue_3 1.0)
                (if false
                  (bind _returnvalue_4 (`CurveFloat.GetFloatValue` (`self.GrappleHookForceCurve`) _time))
                  (`self.DebugMessage` (`KismetStringLibrary.Concat_StrStr` "GrappleHookForce" (`KismetStringLibrary.Conv_DoubleToString` _returnvalue_4))))
                (`CharacterMovementComponent.AddForce` _charactermovement (* (* (* (`KismetMathLibrary.Normal` _returnvalue_2) (`KismetMathLibrary.Dot_VectorVector` (`self.GetVelocity`) _returnvalue_2)) _returnvalue_4) 2.0))
                (set `CharacterMovementComponent.AirControl` (* (`CurveFloat.GetFloatValue` (`self.GrappleHookAirControlCurve`) _returnvalue_3) 2.0) _charactermovement)
                (set `CableComponent.EndLocation` (`KismetMathLibrary.VLerp` _grapplestartinglocation _grapplehookanchorpoint _returnvalue_3) (`self.GrappleHookCable`))
                (`CableComponent.SetAttachEndTo` (`self.GrappleHookCable`) self "None" "None")
                (if (> (`KismetMathLibrary.VSizeSquared` (- (`self.GrappleHookAnchorPoint`) (`self.K2_GetActorLocation`))) (`KismetMathLibrary.Square` (`self.GrappleClosestDistance`)))
                  (if true
                    (bind _returnvalue_5 (* (* (`KismetMathLibrary.Normal` (- _grapplehookanchorpoint _grapplestartinglocation)) (`CurveFloat.GetFloatValue` (`self.GrappleHookRetractSpeedCurve`) _time)) 0.25))
                    (`self.DebugMessage` (`KismetStringLibrary.Concat_StrStr` (`KismetStringLibrary.Concat_StrStr` "[ Velocity: " (`KismetStringLibrary.Conv_DoubleToString` (`KismetMathLibrary.VSize` (`MovementComponent.Velocity` (`self.CharacterMovement`)))) " ] [ " "GrappleHookLaunch") ": " (`KismetStringLibrary.Conv_DoubleToString` (`KismetMathLibrary.VSize` _returnvalue_5)) " ]") true false (struct :`R` 1.0 :`G` 0.15 :`A` 1.0) 2.0))
                  (`self.LaunchCharacter` _returnvalue_5 false false)
                  (else
                    (`self.OnGrappleHookRelease`)))
                (else
                  (`self.OnGrappleHookRelease`)))
              (else
                (goto _label_5 :!via `Stop`)))))))
    (else
      (`|ExecutionSequence`
        (:`then_0`
          (bind (_direction_2 _time_2) (`Timeline|T_GrappleHookLaunch` :!via `Stop` :!label _label_6)
            (:`Update`
              (if (< _time_2 _grapplehookthrowduration)
                (bind _returnvalue_6 (+ _returnvalue (* (`self.GetActorForwardVector` (`GameplayStatics.GetPlayerCameraManager` 0)) (`KismetMathLibrary.Lerp` 0.0 (`self.GrappleHookThrowMaxDistance`) (/ _time_2 _grapplehookthrowduration)))))
                (bind (_outhit _returnvalue_7) (`KismetSystemLibrary.SphereTraceSingle` _returnvalue _returnvalue_6 10.0 "TraceTypeQuery1"))
                (`/Engine/EditorBlueprintResources/StandardMacros.IsValid` _grapplehookanchoractor_3
                  (:`Is Valid`
                    (`SceneComponent.K2_SetWorldLocation` (`Actor.RootComponent` _grapplehookanchoractor_3) _returnvalue_6 false false)
                    (if _returnvalue_7
                      (`|ExecutionSequence`
                        (:`then_0`
                          (bind (_bblockinghit _binitialoverlap _time_3 _distance _location _impactpoint _normal _impactnormal _physmat _hitactor _hitcomponent _hitbonename _hititem _faceindex _tracestart) (`GameplayStatics.BreakHitResult` _outhit))
                          (set `self.GrappleHookAnchorPoint` _impactpoint)
                          (set `self.GrappleStartingLocation` _tracestart)
                          (set `self.GrappleConnected` true)
                          (`SceneComponent.K2_SetWorldLocation` _grapplehookcable _grapplehookanchorpoint_2 false true)
                          (`PrimitiveComponent.SetSimulatePhysics` (`self.CapsuleComponent`) true)
                          (`SceneComponent.SetVisibility` (`self.GrappleHookCable`) true false)
                          (set `CableComponent.EndLocation` _grapplehookanchorpoint_2 (`self.GrappleHookCable`))
                          (`CableComponent.SetAttachEndTo` (`self.GrappleHookCable`) self "None" "None")
                          (goto _label_5 :!via `PlayFromStart`))
                        (:`then_1`
                          (goto _label_6 :!via `Stop`)))))
                  (:`Is Not Valid`
                    (goto _label_6 :!via `Stop`)))
                (else
                  (`self.OnGrappleHookRelease`))))))
        (:`then_1`
          (`/Engine/EditorBlueprintResources/StandardMacros.IsValid` _grapplehookanchoractor
            (:`Is Valid`
              (`self.K2_DestroyActor` _grapplehookanchoractor)
              (goto _label_6 :!via `Stop`))))))))

(fn `AreRequiredKeysDown`
  (returns (AreRequiredKeysDown :type Boolean))
  (bind __frightinputscale (`self._fRightInputScale`))
  (if (> (`self._fForwardInputScale`) 0.1)
    (switch `int` (`self.WallRunEnum`)
      (:`0`
        (return (> __frightinputscale 0.1)))
      (:`1`
        (return (< __frightinputscale -0.1))))
    (else
      (return false))))

(fn `CanSurfaceBeWallRan(GreatePunuation)`
  (params (SurfaceNormal :type "Vector Structure"))
  (returns (`Return Value` :type Boolean))
  (if (< (.z SurfaceNormal) -0.05)
    (return false)
    (else
      (return (< (`KismetMathLibrary.DegAcos` (`KismetMathLibrary.Dot_VectorVector` (`KismetMathLibrary.Normal` (`KismetMathLibrary.MakeVector` (.x SurfaceNormal) (.y SurfaceNormal))) SurfaceNormal)) (`CharacterMovementComponent.K2_GetWalkableFloorAngle` (`self.CharacterMovement`)))))))

(fn `FindLaunchVelocity`
  (returns (LaunchVelocity :type "Vector Structure"))
  (locals (LaunchDirection :type "Vector Structure" :default (0.0 0.0 0.0)))
  (`|ExecutionSequence`
    (:`then_0`
      (if (`self.IsWallRunning_0`)
        (set `local.LaunchDirection` (`KismetMathLibrary.Cross_VectorVector` (`self.WallRunDirection`) (select `int` (`self.WallRunEnum`) :`0` (0.0 0.0 1.0) :`1` (0.0 0.0 -1.0) :!type "Vector Structure")))))
    (:`then_1`
      (return (* (+ (`local.LaunchDirection`) (0.0 0.0 1.0)) (`CharacterMovementComponent.JumpZVelocity` (`self.CharacterMovement`)))))))

(fn `FindRunDirectionAndSide`
  (params (WallNormal :type "Vector Structure"))
  (returns (DirectionVector :type "Vector Structure") (Side :type Integer))
  (locals (SideLocal :type Integer))
  (bind _output_get (set `local.SideLocal` (select `bool` (> (`KismetMathLibrary.DotProduct2D` (`KismetMathLibrary.Conv_VectorToVector2D` WallNormal) (`KismetMathLibrary.Conv_VectorToVector2D` (`self.GetActorRightVector`))) 0.0) :`true` 1)))
  (return (`KismetMathLibrary.Cross_VectorVector` (`local.WallNormal`) (select `int` _output_get :`0` (0.0 0.0 -1.0) :`1` (0.0 0.0 1.0) :!type "Vector Structure")) (`local.SideLocal`)))

(fn `UpdateWallRun`
  (locals (PreviousSide :type Integer))
  (bind _returnvalue (`self.K2_GetActorLocation`))
  (if (`self.AreRequiredKeysDown`)
    (bind (_outhit _returnvalue_2) (`KismetSystemLibrary.LineTraceSingle` _returnvalue (+ _returnvalue (* (`KismetMathLibrary.Cross_VectorVector` (`self.WallRunDirection`) (select `int` (`self.WallRunEnum`) :`0` (0.0 0.0 -1.0) :`1` (0.0 0.0 1.0) :!type "Vector Structure")) 200.0)) "TraceTypeQuery1"))
    (if _returnvalue_2
      (bind (_directionvector _side) (`self.FindRunDirectionAndSide` (`.ImpactNormal` (`GameplayStatics.BreakHitResult` _outhit))))
      (if (== _side (`self.WallRunEnum`))
        (bind _output_get (set `self.WallRunDirection` _directionvector))
        (set `MovementComponent.Velocity` (`KismetMathLibrary.MakeVector` (.x (* _output_get (`MovementComponent.K2_GetModifiedMaxSpeed` (`self.CharacterMovement`)))) (.y (* _output_get (`MovementComponent.K2_GetModifiedMaxSpeed` (`self.CharacterMovement`))))) (`self.CharacterMovement`))))))

(fn `UserConstructionScript`)