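; BP_Door_260x40x360 is an environmental door Blueprint for ArenaShooter that detects Pawns entering and leaving its OpenTrigger component.
; Begin and end overlaps on the trigger cast the other actor to Pawn, then call the OpenDoor or CloseDoor event.
; Both events only print a debug string, so no door movement is implemented here, and pawns inside the trigger are not counted.
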(event `self.OpenTrigger.OnComponentBeginOverlap`
  (params (OverlappedComponent :type "PrimitiveComponent Object Reference") (OtherActor :type "Actor Object Reference") (OtherComp :type "PrimitiveComponent Object Reference") (OtherBodyIndex :type Integer) (bFromSweep :type Boolean) (SweepResult :type "HitResult Structure (by ref)"))
  (if (`.bSuccess` (cast `Pawn` OtherActor :!pure true))
    (`self.OpenDoor`)))

(event `self.OpenTrigger.OnComponentEndOverlap`
  (params (OverlappedComponent :type "PrimitiveComponent Object Reference") (OtherActor :type "Actor Object Reference") (OtherComp :type "PrimitiveComponent Object Reference") (OtherBodyIndex :type Integer))
  (if (`.bSuccess` (cast `Pawn` OtherActor :!pure true))
    (`self.CloseDoor`)))

(event `OpenDoor`
  (`KismetSystemLibrary.PrintString` "Open"))

(event `CloseDoor`
  (`KismetSystemLibrary.PrintString` "Close"))

(fn `UserConstructionScript`)