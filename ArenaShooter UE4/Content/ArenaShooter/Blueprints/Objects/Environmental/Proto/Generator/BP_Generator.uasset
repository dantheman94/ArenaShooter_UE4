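; BP_Generator is a prototype environmental generator object for ArenaShooter, built from a base mesh and two pylon meshes.
; Its construction script adds each mesh to the StaticMeshComponents array if not already present, then runs the parent construction script.
; The event graph holds only disabled placeholder events, so the Blueprint adds no runtime logic of its own.
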(fn `UserConstructionScript`
  (bind _staticmeshcomponents (`self.StaticMeshComponents`))
  (bind _staticmeshcomponents_2 (`self.StaticMeshComponents`))
  (bind _base (`self.Base`))
  (bind _sm_pylon2 (`self.SM_Pylon2`))
  (bind _staticmeshcomponents_3 (`self.StaticMeshComponents`))
  (bind _sm_pylon1 (`self.SM_Pylon1`))
  (`|ExecutionSequence`
    (:`then_0`
      (if (not (`KismetArrayLibrary.Array_Contains` _staticmeshcomponents_2 _base))
        (`KismetArrayLibrary.Array_Add` _staticmeshcomponents_2 _base)))
    (:`then_1`
      (if (not (`KismetArrayLibrary.Array_Contains` _staticmeshcomponents_3 _sm_pylon1))
        (`KismetArrayLibrary.Array_Add` _staticmeshcomponents_3 _sm_pylon1)))
    (:`then_2`
      (if (not (`KismetArrayLibrary.Array_Contains` _staticmeshcomponents _sm_pylon2))
        (`KismetArrayLibrary.Array_Add` _staticmeshcomponents _sm_pylon2)))
    (:`then_3`
      (`parent.UserConstructionScript`))))