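; Prototype environment actor that tints its static mesh components with a two-colour palette.
; The construction script and a RegenerateColourPalette event apply PrimaryColour and SecondaryColour through dynamic instances of MI_ProtoTools_Blue on slot 0 of each mesh.
; With UseRandomColourPalette set, both first take the colours from a random row of the DTColourPalettes data table.
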(event `RegenerateColourPalette`
  (if (`self.UseRandomColourPalette`)
    (`self.f_GetRandomColourPaletteFromTable`))
  (for _array_element (`self.StaticMeshComponents`)
    (bind _returnvalue (`PrimitiveComponent.CreateDynamicMaterialInstance` _array_element 0 "/Game/External/ProtoTools/Materials/Instances/MI_ProtoTools_Blue.MI_ProtoTools_Blue" "None"))
    (`MaterialInstanceDynamic.SetVectorParameterValue` _returnvalue "BaseColor" (`self.PrimaryColour`))
    (`MaterialInstanceDynamic.SetVectorParameterValue` _returnvalue "BaseColor2" (`self.SecondaryColour`))))

(fn `f_GetRandomColourPaletteFromTable`
  (locals (iter :type Integer) (RowName :type Name))
  (bind _dt_colourpalettes (`self.DT_ColourPalettes`))
  (`/Engine/EditorBlueprintResources/StandardMacros.IsValid` _dt_colourpalettes
    (:`Is Valid`
      (bind _outrownames (`DataTableFunctionLibrary.GetDataTableRowNames` _dt_colourpalettes))
      (set `local.iter` (`KismetMathLibrary.RandomIntegerInRange` 0 (- (`KismetArrayLibrary.Array_Length` _outrownames) 1)))
      (for (_array_element _array_index) _outrownames
        (if (== _array_index (`local.iter`))
          (set `local.RowName` _array_element)
          (break)))
      (bind _returnvalue (`|GetDataTableRow` (`self.DT_ColourPalettes`) (`local.RowName`))
        (:`then`
          (bind (_primarycolour _secondarycolour) (break `/Game/ArenaShooter/Blueprints/Objects/Environmental/Proto/F_ProtoColourPalette` _returnvalue))
          (set `self.PrimaryColour` _primarycolour)
          (set `self.SecondaryColour` _secondarycolour))
        (:`RowNotFound`
          _)))
    (:`Is Not Valid`
      _))
  (return))

(fn `UserConstructionScript`
  (if (`self.UseRandomColourPalette`)
    (`self.f_GetRandomColourPaletteFromTable`))
  (for _array_element (`self.StaticMeshComponents`)
    (bind _returnvalue (`PrimitiveComponent.CreateDynamicMaterialInstance` _array_element 0 "/Game/External/ProtoTools/Materials/Instances/MI_ProtoTools_Blue.MI_ProtoTools_Blue" "None"))
    (`MaterialInstanceDynamic.SetVectorParameterValue` _returnvalue "BaseColor" (`self.PrimaryColour`))
    (`MaterialInstanceDynamic.SetVectorParameterValue` _returnvalue "BaseColor2" (`self.SecondaryColour`))))