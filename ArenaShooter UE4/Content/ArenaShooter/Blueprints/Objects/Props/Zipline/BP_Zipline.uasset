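; Zipline prop that strings a cable between two pole heads, with optional visibility for each pole.
; The construction script and Tick both turn the heads toward each other, attach the cable between them, set its length to their distance and apply pole visibility.
; Tick also places the interaction trigger from stored location and rotation variables; nodes that derive it from the head positions are disconnected, and no riding logic is here.
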(event `self.ReceiveTick`
  (params (DeltaSeconds :type "Float (single-precision)"))
  (bind _ziplinecable (`self.ZiplineCable`))
  (bind _zipline1rootchild (`self.Zipline1RootChild`))
  (bind _zipline2rootchild (`self.Zipline2RootChild`))
  (bind _returnvalue (`SceneComponent.K2_GetComponentLocation` (`self.SM_Zipline2Head`)))
  (bind _returnvalue_2 (`SceneComponent.K2_GetComponentLocation` (`self.SM_Zipline1Head`)))
  (bind _returnvalue_3 (`SceneComponent.K2_GetComponentLocation` (`self.SM_Zipline1Head`)))
  (`SceneComponent.K2_SetWorldRotation` (`self.SM_Zipline1Head`) (* (`KismetMathLibrary.FindLookAtRotation` _returnvalue_2 _returnvalue) 90) false false)
  (`SceneComponent.K2_SetWorldRotation` (`self.SM_Zipline2Head`) (* (`KismetMathLibrary.FindLookAtRotation` _returnvalue _returnvalue_2) 90) false false)
  (set `CableComponent.bAttachStart` true _ziplinecable)
  (`SceneComponent.K2_SetWorldLocation` _ziplinecable _returnvalue_3 false false)
  (set `CableComponent.bAttachEnd` true _ziplinecable)
  (`CableComponent.SetAttachEndTo` _ziplinecable self "SM_Zipline2Head" "Head")
  (set `CableComponent.CableLength` (`KismetMathLibrary.Vector_Distance` _returnvalue_3 (`SceneComponent.K2_GetComponentLocation` (`self.SM_Zipline2Head`))) (`self.ZiplineCable`))
  (`SceneComponent.K2_SetWorldLocationAndRotation` (`self.Trigger_CableInteraction`) (`self.InteractionTriggerLocation`) (`self.InteractionTriggerRotation`) false false)
  (`|ExecutionSequence`
    (:`then_0`
      (`SceneComponent.SetHiddenInGame` _zipline1rootchild (not (`self.Show_Pole1`)) true)
      (`SceneComponent.SetVisibility` _zipline1rootchild (`self.Show_Pole1`) true))
    (:`then_1`
      (`SceneComponent.SetHiddenInGame` _zipline2rootchild (not (`self.Show_Pole2`)) true)
      (`SceneComponent.SetVisibility` _zipline2rootchild (`self.Show_Pole2`) true))))

(fn `UserConstructionScript`
  (bind _ziplinecable (`self.ZiplineCable`))
  (bind _zipline1rootchild (`self.Zipline1RootChild`))
  (bind _zipline2rootchild (`self.Zipline2RootChild`))
  (bind _returnvalue (`SceneComponent.K2_GetComponentLocation` (`self.SM_Zipline2Head`)))
  (bind _returnvalue_2 (`SceneComponent.K2_GetComponentLocation` (`self.SM_Zipline1Head`)))
  (`SceneComponent.K2_SetWorldRotation` (`self.SM_Zipline1Head`) (* (`KismetMathLibrary.FindLookAtRotation` _returnvalue_2 _returnvalue) 90) false false)
  (`SceneComponent.K2_SetWorldRotation` (`self.SM_Zipline2Head`) (* (`KismetMathLibrary.FindLookAtRotation` _returnvalue _returnvalue_2) 90) false false)
  (set `CableComponent.bAttachStart` true _ziplinecable)
  (`SceneComponent.K2_SetWorldLocation` _ziplinecable (`SceneComponent.K2_GetComponentLocation` (`self.SM_Zipline1Head`)) false false)
  (set `CableComponent.bAttachEnd` true _ziplinecable)
  (`CableComponent.SetAttachEndTo` _ziplinecable self "SM_Zipline2Head" "Head")
  (set `CableComponent.CableLength` (`KismetMathLibrary.Vector_Distance` (`SceneComponent.K2_GetComponentLocation` (`self.SM_Zipline1Head`)) (`SceneComponent.K2_GetComponentLocation` (`self.SM_Zipline2Head`))) (`self.ZiplineCable`))
  (`|ExecutionSequence`
    (:`then_0`
      (`SceneComponent.SetHiddenInGame` _zipline1rootchild (not (`self.Show_Pole1`)) true)
      (`SceneComponent.SetVisibility` _zipline1rootchild (`self.Show_Pole1`) true))
    (:`then_1`
      (`SceneComponent.SetHiddenInGame` _zipline2rootchild (not (`self.Show_Pole2`)) true)
      (`SceneComponent.SetVisibility` _zipline2rootchild (`self.Show_Pole2`) true))))