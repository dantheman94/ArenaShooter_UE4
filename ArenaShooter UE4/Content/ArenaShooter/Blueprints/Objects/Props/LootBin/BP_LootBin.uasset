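; Loot bin prop that, on interaction, fills three child-actor slots with weapons and swings its lid open on a timeline.
; Weapons are preset or drawn from a DataTable, where spawn weights are collected but the pick is uniformly random.
; Spawned weapons have physics disabled and empty their slot when taken.
; OnReps toggle the interaction lock, but nothing here starts closing and the open/closed timers trigger nothing on expiry.
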(event `self.BP_InteractionData.OnInteract`
  (`self.Spawn Weapons`)
  (`self.StartOpeningDoor`))

(event `self.ReceiveBeginPlay`
  (`self.ClearWeapons`)
  (`self.BindEventToOnDoorOpened`)
  (`self.BindEventToOnDoorOpened`))

(event `Clear Weapons`
  (`self.ClearWeapons`))

(event `Spawn Weapons`
  (`self.Clear Weapons`)
  (if (`self.RandomLoot`)
    (`self.GenerateRandomLoot`)
    (else
      (`self.SetWeapons` (`self.Weapon_1`) (`self.Weapon_2`) (`self.Weapon_3`)))))

(event `StartOpeningDoor`
  (set `self.fDoorOpenAlpha` 0.0)
  (bind (_direction _time) (`Timeline|T_DoorOpenUpdate` :!via `PlayFromStart` :!label _label)
    (:`Update`
      (bind _output_get (set `self.fDoorOpenAlpha` (`KismetMathLibrary.FClamp` (/ _time (`self.fTimeToOpenDoor`)))))
      (if (>= (`KismetMathLibrary.NormalizeToRange` _output_get 0.0 (`self.fMaxDoorOpenAlpha`)) 1.0)
        (`|ExecutionSequence`
          (:`then_0`
            (`self.OnDoorOpened`))
          (:`then_1`
            (goto _label :!via `Stop`)))
        (else
          (`SceneComponent.K2_SetRelativeRotation` (`self.PIVOT_Head`) (`KismetMathLibrary.RLerp` (`self.ROT_DoorClosed`) (`self.ROT_DoorOpened`) (`self.fDoorOpenAlpha`)) false false))))))

(event `SetWeapons`
  (params (`Weapon 1` :type "/Game/ArenaShooter/Blueprints/Objects/Weapon/BP_InteractableWeapon Class Reference") (`Weapon 2` :type "/Game/ArenaShooter/Blueprints/Objects/Weapon/BP_InteractableWeapon Class Reference") (`Weapon 3` :type "/Game/ArenaShooter/Blueprints/Objects/Weapon/BP_InteractableWeapon Class Reference"))
  (bind _weapon_l (`self.Weapon_L`))
  (bind _weapon_m (`self.Weapon_M`))
  (bind _weapon_r (`self.Weapon_R`))
  (`self.ClearWeapons`)
  (if (`KismetSystemLibrary.IsValidClass` `Weapon 1`)
    (`ChildActorComponent.SetChildActorClass` _weapon_l `Weapon 1`)
    (bind _asbp_interactable_weapon (cast `/Game/ArenaShooter/Blueprints/Objects/Weapon/BP_InteractableWeapon` (`ChildActorComponent.ChildActor` _weapon_l))
      (:`then`
        (bind __interactiondata (`InteractableWeapon._InteractionData` _asbp_interactable_weapon))
        (`InteractionDataComponent.SetSimulatePhysicsOnStart` __interactiondata false)
        (`PrimitiveComponent.SetSimulatePhysics` (`InteractableWeapon._WeaponMesh` _asbp_interactable_weapon) (`InteractionDataComponent._bSimulatePhysicsOnStart` __interactiondata)))
      (:`CastFailed`
        _)))
  (if (`KismetSystemLibrary.IsValidClass` `Weapon 2`)
    (`ChildActorComponent.SetChildActorClass` _weapon_m `Weapon 2`)
    (bind _asbp_interactable_weapon_2 (cast `/Game/ArenaShooter/Blueprints/Objects/Weapon/BP_InteractableWeapon` (`ChildActorComponent.ChildActor` _weapon_m))
      (:`then`
        (bind __interactiondata_2 (`InteractableWeapon._InteractionData` _asbp_interactable_weapon_2))
        (`InteractionDataComponent.SetSimulatePhysicsOnStart` __interactiondata_2 false)
        (`PrimitiveComponent.SetSimulatePhysics` (`InteractableWeapon._WeaponMesh` _asbp_interactable_weapon_2) (`InteractionDataComponent._bSimulatePhysicsOnStart` __interactiondata_2)))
      (:`CastFailed`
        _)))
  (if (`KismetSystemLibrary.IsValidClass` `Weapon 3`)
    (`ChildActorComponent.SetChildActorClass` _weapon_r `Weapon 3`)
    (bind _asbp_interactable_weapon_3 (cast `/Game/ArenaShooter/Blueprints/Objects/Weapon/BP_InteractableWeapon` (`ChildActorComponent.ChildActor` _weapon_r))
      (:`then`
        (bind __interactiondata_3 (`InteractableWeapon._InteractionData` _asbp_interactable_weapon_3))
        (`InteractionDataComponent.SetSimulatePhysicsOnStart` __interactiondata_3 false)
        (`PrimitiveComponent.SetSimulatePhysics` (`InteractableWeapon._WeaponMesh` _asbp_interactable_weapon_3) (`InteractionDataComponent._bSimulatePhysicsOnStart` __interactiondata_3)))
      (:`CastFailed`
        _)))
  (bind _asbp_interactable_weapon_4 (cast `/Game/ArenaShooter/Blueprints/Objects/Weapon/BP_InteractableWeapon` (`ChildActorComponent.ChildActor` (`self.Weapon_L`)))
    (:`then`
      (add `InteractionDataComponent.OnInteract` (`InteractableWeapon._InteractionData` _asbp_interactable_weapon_4) (delegate `OnInteract_ItemLeft`)))
    (:`CastFailed`
      _))
  (bind _asbp_interactable_weapon_5 (cast `/Game/ArenaShooter/Blueprints/Objects/Weapon/BP_InteractableWeapon` (`ChildActorComponent.ChildActor` (`self.Weapon_M`)))
    (:`then`
      (add `InteractionDataComponent.OnInteract` (`InteractableWeapon._InteractionData` _asbp_interactable_weapon_5) (delegate `OnInteract_ItemMiddle`)))
    (:`CastFailed`
      _))
  (bind _asbp_interactable_weapon_6 (cast `/Game/ArenaShooter/Blueprints/Objects/Weapon/BP_InteractableWeapon` (`ChildActorComponent.ChildActor` (`self.Weapon_R`))))
  (add `InteractionDataComponent.OnInteract` (`InteractableWeapon._InteractionData` _asbp_interactable_weapon_6) (delegate `OnInteract_ItemRight`)))

(event `StartClosingDoor`
  (set `self.StartingDoorRotation` (`SceneComponent.RelativeRotation` (`self.PIVOT_Head`)))
  (set `self.fDoorOpenAlpha` 0.0)
  (bind (_direction _time) (`Timeline|T_DoorCloseUpdate` :!via `PlayFromStart` :!label _label_2)
    (:`Update`
      (bind _output_get (set `self.fDoorOpenAlpha` (`KismetMathLibrary.FClamp` (/ _time (`self.fTimeToOpenDoor`)))))
      (if (>= _output_get 1.0)
        (`|ExecutionSequence`
          (:`then_0`
            (`self.OnDoorClosed`))
          (:`then_1`
            (goto _label_2 :!via `Stop`)))
        (else
          (`SceneComponent.K2_SetRelativeRotation` (`self.PIVOT_Head`) (`KismetMathLibrary.RLerp` (`self.StartingDoorRotation`) (`self.ROT_DoorClosed`) (`self.fDoorOpenAlpha`)) false false))))))

(event `OnInteract_ItemMiddle`
  (`KismetSystemLibrary.PrintString` "Hello")
  (`ChildActorComponent.SetChildActorClass` (`self.Weapon_M`) null))

(event `OnInteract_ItemRight`
  (`KismetSystemLibrary.PrintString` "Hello")
  (`ChildActorComponent.SetChildActorClass` (`self.Weapon_R`) null))

(event `OnInteract_ItemLeft`
  (`KismetSystemLibrary.PrintString` "Hello")
  (`ChildActorComponent.SetChildActorClass` (`self.Weapon_L`) null))

(event `BindEventToOnDoorOpened`
  (add `self.OnDoorOpened` (delegate `StartDoorOpenedTimer`)))

(event `StartDoorOpenedTimer`
  (set `self.fOpenDoorTimerPos` 0.0)
  (`Timeline|T_UpdateDoorOpenedTimer` :!label _label_3
    (:`Update`
      (bind _output_get (set `self.fOpenDoorTimerPos` (+ (`self.fOpenDoorTimerPos`) (`GameplayStatics.GetWorldDeltaSeconds`))))
      (if (>= _output_get (`self.fDoorOpenTime`))
        (`|ExecutionSequence`
          (:`then_1`
            (goto _label_3 :!via `Stop`)))))))

(event `BindEventToOnDoorClosed`
  (add `self.OnDoorClosed` (delegate `StartDoorClosedTimer`)))

(event `StartDoorClosedTimer`
  (set `self.fClosedDoorTimerPos` 0.0)
  (`self.ClearWeapons`)
  (`Timeline|T_UpdateDoorClosedTimer` :!label _label_4
    (:`Update`
      (bind _output_get (set `self.fClosedDoorTimerPos` (+ (`self.fClosedDoorTimerPos`) (`GameplayStatics.GetWorldDeltaSeconds`))))
      (if (>= _output_get (`self.fDoorClosedTime`))
        (`|ExecutionSequence`
          (:`then_1`
            (goto _label_4 :!via `Stop`)))))))

(fn `f_GetRandomIntFromDataTable`
  (returns (Output :type Integer))
  (locals (OutInt :type Integer) (Weights :type "Array of Integer"))
  (`/Engine/EditorBlueprintResources/StandardMacros.IsValid` (`self.DataTable`)
    (:`Is Valid`
      (bind _outrownames (`DataTableFunctionLibrary.GetDataTableRowNames` (`self.DataTable`)))
      (for _array_element _outrownames
        (bind _returnvalue (`|GetDataTableRow` (`self.DataTable`) _array_element)
          (:`then`
            (`KismetArrayLibrary.Array_Add` (`local.Weights`) (`.SpawnWeight_7_910E9C17405826C40B225EB89A07DFCC` (break `/Game/ArenaShooter/Blueprints/Objects/Props/LootBin/FWeaponLootRate` _returnvalue))))))
      (bind _outint (`self.GetWeightedIntFromList` (`local.Weights`)))
      (set `local.OutInt` _outint))
    (:`Is Not Valid`
      (set `local.OutInt` 0)))
  (return (`local.OutInt`)))

(fn `f_GetWeaponByInt`
  (params (Input :type Integer))
  (returns (InteractableWeapon :type "/Game/ArenaShooter/Blueprints/Objects/Weapon/BP_InteractableWeapon Class Reference"))
  (locals (Weapon :type "/Game/ArenaShooter/Blueprints/Objects/Weapon/BP_InteractableWeapon Class Reference"))
  (`/Engine/EditorBlueprintResources/StandardMacros.IsValid` (`self.DataTable`)
    (:`Is Valid`
      (bind _outrownames (`DataTableFunctionLibrary.GetDataTableRowNames` (`self.DataTable`)))
      (for (_array_element _array_index) _outrownames
        (bind _returnvalue (`|GetDataTableRow` (`self.DataTable`) _array_element)
          (:`then`
            (if (== _array_index Input)
              (set `local.Weapon` (`.Weapon_9_B012ACD6477EDA80DB82DCB290BAD721` (break `/Game/ArenaShooter/Blueprints/Objects/Props/LootBin/FWeaponLootRate` _returnvalue)))
              (break))))))
    (:`Is Not Valid`
      (set `local.Weapon` null)))
  (return (`local.Weapon`)))

(fn `OnRep_OnDoorClosed`
  (`InteractionDataComponent.SetIsLocked` (`self.BP_InteractionData`) false))

(fn `OnRep_OnDoorOpened`
  (`InteractionDataComponent.SetIsLocked` (`self.BP_InteractionData`) true))

(fn `UserConstructionScript`
  (set `self.fDoorOpenAlpha` (`KismetMathLibrary.FClamp` (`self.fDoorOpenAlpha`) 0.0 (`self.fMaxDoorOpenAlpha`)))
  (`SceneComponent.K2_SetRelativeRotation` (`self.PIVOT_Head`) (`KismetMathLibrary.RLerp` (`self.ROT_DoorClosed`) (`self.ROT_DoorOpened`) (`self.fDoorOpenAlpha`)) false false))