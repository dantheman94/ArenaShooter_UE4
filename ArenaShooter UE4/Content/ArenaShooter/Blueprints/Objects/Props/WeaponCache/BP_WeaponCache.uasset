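; Weapon cache prop for the arena shooter that holds six configurable weapons and triggers its opening a set number of seconds into the match.
; The construction script assigns a class to each child actor slot, A1–A3 and B1–B3, and turns off physics on each interactable weapon.
; BeginPlay waits for the delay, then calls PlayOpenAnimation, an event with an empty body here.
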(event `self.ReceiveBeginPlay`
  (`KismetSystemLibrary.Delay` (`self.InitiateSecondsIntoTheMatch`))
  (`self.PlayOpenAnimation`))

(event `PlayOpenAnimation`)

(event `SetWeapons`
  (bind _bp_weaponb2 (`self.BP_WeaponB2`))
  (bind _bp_weapona1 (`self.BP_WeaponA1`))
  (bind _bp_weapona2 (`self.BP_WeaponA2`))
  (bind _bp_weapona3 (`self.BP_WeaponA3`))
  (bind _bp_weaponb1 (`self.BP_WeaponB1`))
  (bind _bp_weaponb3 (`self.BP_WeaponB3`))
  (`ChildActorComponent.SetChildActorClass` _bp_weapona1 (`self.WeaponA1`))
  (bind _asbp_interactable_weapon (cast `/Game/ArenaShooter/Blueprints/Objects/Weapon/BP_InteractableWeapon` (`ChildActorComponent.ChildActor` _bp_weapona1))
    (:`then`
      (bind __interactiondata (`InteractableWeapon._InteractionData` _asbp_interactable_weapon))
      (`InteractionDataComponent.SetSimulatePhysicsOnStart` __interactiondata false)
      (`PrimitiveComponent.SetSimulatePhysics` (`InteractableWeapon._WeaponMesh` _asbp_interactable_weapon) (`InteractionDataComponent._bSimulatePhysicsOnStart` __interactiondata)))
    (:`CastFailed`
      _))
  (`ChildActorComponent.SetChildActorClass` _bp_weapona2 (`self.WeaponA2`))
  (bind _asbp_interactable_weapon_2 (cast `/Game/ArenaShooter/Blueprints/Objects/Weapon/BP_InteractableWeapon` (`ChildActorComponent.ChildActor` _bp_weapona2))
    (:`then`
      (bind __interactiondata_2 (`InteractableWeapon._InteractionData` _asbp_interactable_weapon_2))
      (`InteractionDataComponent.SetSimulatePhysicsOnStart` __interactiondata_2 false)
      (`PrimitiveComponent.SetSimulatePhysics` (`InteractableWeapon._WeaponMesh` _asbp_interactable_weapon_2) (`InteractionDataComponent._bSimulatePhysicsOnStart` __interactiondata_2)))
    (:`CastFailed`
      _))
  (`ChildActorComponent.SetChildActorClass` _bp_weapona3 (`self.WeaponA3`))
  (bind _asbp_interactable_weapon_3 (cast `/Game/ArenaShooter/Blueprints/Objects/Weapon/BP_InteractableWeapon` (`ChildActorComponent.ChildActor` _bp_weapona3))
    (:`then`
      (bind __interactiondata_3 (`InteractableWeapon._InteractionData` _asbp_interactable_weapon_3))
      (`InteractionDataComponent.SetSimulatePhysicsOnStart` __interactiondata_3 false)
      (`PrimitiveComponent.SetSimulatePhysics` (`InteractableWeapon._WeaponMesh` _asbp_interactable_weapon_3) (`InteractionDataComponent._bSimulatePhysicsOnStart` __interactiondata_3)))
    (:`CastFailed`
      _))
  (`ChildActorComponent.SetChildActorClass` _bp_weaponb1 (`self.WeaponB1`))
  (bind _asbp_interactable_weapon_4 (cast `/Game/ArenaShooter/Blueprints/Objects/Weapon/BP_InteractableWeapon` (`ChildActorComponent.ChildActor` _bp_weaponb1))
    (:`then`
      (bind __interactiondata_4 (`InteractableWeapon._InteractionData` _asbp_interactable_weapon_4))
      (`InteractionDataComponent.SetSimulatePhysicsOnStart` __interactiondata_4 false)
      (`PrimitiveComponent.SetSimulatePhysics` (`InteractableWeapon._WeaponMesh` _asbp_interactable_weapon_4) (`InteractionDataComponent._bSimulatePhysicsOnStart` __interactiondata_4)))
    (:`CastFailed`
      _))
  (`ChildActorComponent.SetChildActorClass` _bp_weaponb2 (`self.WeaponB2`))
  (bind _asbp_interactable_weapon_5 (cast `/Game/ArenaShooter/Blueprints/Objects/Weapon/BP_InteractableWeapon` (`ChildActorComponent.ChildActor` _bp_weaponb2))
    (:`then`
      (bind __interactiondata_5 (`InteractableWeapon._InteractionData` _asbp_interactable_weapon_5))
      (`InteractionDataComponent.SetSimulatePhysicsOnStart` __interactiondata_5 false)
      (`PrimitiveComponent.SetSimulatePhysics` (`InteractableWeapon._WeaponMesh` _asbp_interactable_weapon_5) (`InteractionDataComponent._bSimulatePhysicsOnStart` __interactiondata_5)))
    (:`CastFailed`
      _))
  (`ChildActorComponent.SetChildActorClass` _bp_weaponb3 (`self.WeaponB3`))
  (bind _asbp_interactable_weapon_6 (cast `/Game/ArenaShooter/Blueprints/Objects/Weapon/BP_InteractableWeapon` (`ChildActorComponent.ChildActor` _bp_weaponb3)))
  (bind __interactiondata_6 (`InteractableWeapon._InteractionData` _asbp_interactable_weapon_6))
  (`InteractionDataComponent.SetSimulatePhysicsOnStart` __interactiondata_6 false)
  (`PrimitiveComponent.SetSimulatePhysics` (`InteractableWeapon._WeaponMesh` _asbp_interactable_weapon_6) (`InteractionDataComponent._bSimulatePhysicsOnStart` __interactiondata_6)))

(fn `UserConstructionScript`
  (`self.SetWeapons`))