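; Short shipping container prop with two lockable doors that pawns push open or shut by walking into them.
; Door hits step each pivot's yaw by push speed and frame delta within clamped limits, with world hit normal Y choosing direction and printing debug text.
; The construction script applies door angles and lock labels, then sets either the default material or, behind a DoOnce, a random data table colour.
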(event `self.SM_Door_a.OnComponentHit`
  (params (HitComponent :type "PrimitiveComponent Object Reference") (OtherActor :type "Actor Object Reference") (OtherComp :type "PrimitiveComponent Object Reference") (NormalImpulse :type "Vector Structure") (Hit :type "HitResult Structure (by ref)"))
  (bind (_bblockinghit _binitialoverlap _time _distance _location _impactpoint _normal _impactnormal _physmat _hitactor) (`GameplayStatics.BreakHitResult` Hit))
  (bind _doorpushspeed (`self.DoorPushSpeed`))
  (if (not (`self.bDoorALocked`))
    (cast `Pawn` _hitactor)
    (if (>= (.y _normal) 0.0)
      (`KismetSystemLibrary.PrintString` "Hit_outside" true false)
      (bind _output_get (set `self.fDoorARotation` (+ (`self.fDoorARotation`) (* (`GameplayStatics.GetWorldDeltaSeconds`) _doorpushspeed))))
      (`SceneComponent.K2_SetRelativeRotation` (`self.PIVOT_Door_a`) (`KismetMathLibrary.MakeRotator` 0.0 0.0 (`KismetMathLibrary.FClamp` _output_get -85.0 255.0)) false false)
      (else
        (`KismetSystemLibrary.PrintString` "Hit_inside" true false (struct :`R` 0.66 :`A` 1.0))
        (bind _output_get_2 (set `self.fDoorARotation` (- (`self.fDoorARotation`) (* (`GameplayStatics.GetWorldDeltaSeconds`) _doorpushspeed))))
        (`SceneComponent.K2_SetRelativeRotation` (`self.PIVOT_Door_a`) (`KismetMathLibrary.MakeRotator` 0.0 0.0 (`KismetMathLibrary.FClamp` _output_get_2 -85.0 255.0)) false false)))))

(event `self.SM_Door_b.OnComponentHit`
  (params (HitComponent :type "PrimitiveComponent Object Reference") (OtherActor :type "Actor Object Reference") (OtherComp :type "PrimitiveComponent Object Reference") (NormalImpulse :type "Vector Structure") (Hit :type "HitResult Structure (by ref)"))
  (bind (_bblockinghit _binitialoverlap _time _distance _location _impactpoint _normal _impactnormal _physmat _hitactor) (`GameplayStatics.BreakHitResult` Hit))
  (bind _doorpushspeed (`self.DoorPushSpeed`))
  (if (not (`self.bDoorBLocked`))
    (cast `Pawn` _hitactor)
    (if (>= (.y _normal) 0.0)
      (`KismetSystemLibrary.PrintString` "Hit_outside" true false)
      (bind _output_get (set `self.fDoorBRotation` (+ (`self.fDoorBRotation`) (* (`GameplayStatics.GetWorldDeltaSeconds`) _doorpushspeed))))
      (`SceneComponent.K2_SetRelativeRotation` (`self.PIVOT_Door_b`) (`KismetMathLibrary.MakeRotator` 0.0 0.0 (`KismetMathLibrary.FClamp` _output_get -255.0 85.0)) false false)
      (else
        (`KismetSystemLibrary.PrintString` "Hit_inside" true false (struct :`R` 0.66 :`A` 1.0))
        (bind _output_get_2 (set `self.fDoorBRotation` (- (`self.fDoorBRotation`) (* (`GameplayStatics.GetWorldDeltaSeconds`) _doorpushspeed))))
        (`SceneComponent.K2_SetRelativeRotation` (`self.PIVOT_Door_b`) (`KismetMathLibrary.MakeRotator` 0.0 0.0 (`KismetMathLibrary.FClamp` _output_get_2 -255.0 85.0)) false false)))))

(fn `UserConstructionScript`
  (locals (LockedText :type Text :default "NSLOCTEXT(\"\", \"36A3DBE24521D9528BABE1B1699A2CC0\", \"Locked\")") (UnlockedText :type Text :default "NSLOCTEXT(\"\", \"02EBC5D042E28AE884919A9B179E5AB5\", \"Unlocked\")"))
  (bind _text_debugdoorblocked1 (`self.TEXT_DebugDoorBLocked1`))
  (bind _text_debugdooralocked1 (`self.TEXT_DebugDoorALocked1`))
  ;[1 1 1] Rotate Doors
  (`SceneComponent.K2_SetRelativeRotation` (`self.PIVOT_Door_a`) (`KismetMathLibrary.MakeRotator` 0.0 0.0 (`KismetMathLibrary.FClamp` (`self.fDoorARotation`) -85.0 255.0)) false false)
  (`SceneComponent.K2_SetRelativeRotation` (`self.PIVOT_Door_b`) (`KismetMathLibrary.MakeRotator` 0.0 0.0 (`KismetMathLibrary.FClamp` (`self.fDoorBRotation`) -255.0 85.0)) false false)
  ;[1 1 1] Door Locked/Unlocked text
  (if (`self.bDoorALocked`)
    (`TextRenderComponent.K2_SetText` _text_debugdooralocked1 (`local.LockedText`))
    (`TextRenderComponent.K2_SetText` (`self.TEXT_DebugDoorALocked2`) (`local.LockedText`))
    (else
      (`TextRenderComponent.K2_SetText` _text_debugdooralocked1 (`local.UnlockedText`))
      (`TextRenderComponent.K2_SetText` (`self.TEXT_DebugDoorALocked2`) (`local.UnlockedText`))))
  (if (`self.bDoorBLocked`)
    (`TextRenderComponent.K2_SetText` _text_debugdoorblocked1 (`local.LockedText`))
    (`TextRenderComponent.K2_SetText` (`self.TEXT_DebugDoorBLocked2`) (`local.LockedText`))
    (else
      (`TextRenderComponent.K2_SetText` _text_debugdoorblocked1 (`local.UnlockedText`))
      (`TextRenderComponent.K2_SetText` (`self.TEXT_DebugDoorBLocked2`) (`local.UnlockedText`))))
  ;[1 1 1] Container Colour
  (if (`self.bRandomContainerColour`)
    (`/Engine/EditorBlueprintResources/StandardMacros.DoOnce` false :!label _label
      (:`Completed`
        (bind _outrownames (`DataTableFunctionLibrary.GetDataTableRowNames` (`self.DT_ColourTable`)))
        (bind _returnvalue (`|GetDataTableRow` (`self.DT_ColourTable`) (`|GetArrayItem` _outrownames (`KismetMathLibrary.RandomIntegerInRange` 0 (- (`KismetArrayLibrary.Array_Length` _outrownames) 1))))
          (:`then`
            (bind (_r _g _b) (break `LinearColor` (`.ColourData_10_07A29A934358F9D6E3C36995A6CE9548` (break `/Game/ArenaShooter/Blueprints/Objects/Props/Crates/S_ColourMaterials` _returnvalue))))
            (`MeshComponent.SetVectorParameterValueOnMaterials` (`self.SM_Interior`) "Colour" (`KismetMathLibrary.MakeVector` _r _g _b))))))
    (else
      (`|ExecutionSequence`
        (:`then_0`
          (goto _label :!via `Reset`))
        (:`then_1`
          (`PrimitiveComponent.SetMaterial` (`self.SM_Interior`) 0 (`self.ContainerMaterial`)))))))