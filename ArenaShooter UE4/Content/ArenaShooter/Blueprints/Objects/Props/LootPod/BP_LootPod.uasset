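; Loot pod prop that lands in the arena after a delay into the match and opens to offer three configurable weapons.
; Timelines act as update loops, growing the body from zero scale while moving it backwards along a spline to its first point.
; A float curve sets descent speed from the remaining straight-line distance.
; After landing, UpdateDoors spawns weapon child actors and offsets three doors; the Construction Script also calls it.
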(event `self.ReceiveBeginPlay`
  (`KismetSystemLibrary.Delay` (`self.InitiateSecondsIntoTheMatch`))
  (`self.StartLandingProcedure`))

(event `StartLandingProcedure`
  (bind _spl_landingpath (`self.SPL_LandingPath`))
  (bind _scale (`self.Scale`))
  (bind _returnvalue (`SplineComponent.GetLocationAtSplinePoint` _spl_landingpath 0 "World"))
  (bind _returnvalue_2 (/ _scale (`self.TimeToReachFullScale`)))
  (bind _output_get (set `self.Scale` 0.0))
  (`SceneComponent.SetWorldScale3D` (`self.SM_Body`) (`KismetMathLibrary.MakeVector` _output_get _output_get _output_get))
  (`|ExecutionSequence`
    (:`then_0`
      (`SceneComponent.K2_SetWorldLocation` (`self.LootPodRootChild`) (`SplineComponent.GetLocationAtSplinePoint` _spl_landingpath (`SplineComponent.GetNumberOfSplinePoints` _spl_landingpath) "World") false false)
      (set `self.DistanceAlongSpline` (`KismetMathLibrary.Vector_Distance` (`SceneComponent.K2_GetComponentLocation` (`self.SM_Body`)) _returnvalue))
      (`Timeline|TimelineUpdate` :!label _label
        (:`Update`
          (bind _output_get_2 (set `self.DistanceAlongSpline` (- (`self.DistanceAlongSpline`) (* (`GameplayStatics.GetWorldDeltaSeconds`) (`CurveFloat.GetFloatValue` (`self.LandingSpeed`) (`KismetMathLibrary.Vector_Distance` (`SceneComponent.K2_GetComponentLocation` (`self.SM_Body`)) _returnvalue))))))
          (`KismetSystemLibrary.PrintString` (`KismetStringLibrary.Conv_DoubleToString` _output_get_2) false false)
          (if (> _output_get_2 0.0)
            (`SceneComponent.K2_SetWorldLocation` (`self.LootPodRootChild`) (`SplineComponent.GetLocationAtDistanceAlongSpline` (`self.SPL_LandingPath`) (`self.DistanceAlongSpline`) "World") false false)
            (else
              (`|ExecutionSequence`
                (:`then_0`
                  (`/Engine/EditorBlueprintResources/StandardMacros.DoOnce` false
                    (:`Completed`
                      (`KismetSystemLibrary.Delay` 3.0)
                      (set `self.bIsOpen` true)
                      (`self.UpdateDoors`))))
                (:`then_1`
                  (goto _label :!via `Stop`))))))))
    (:`then_1`
      (`Timeline|T_TimelineUpdate2`
        (:`Update`
          (set `self.Scale` (+ (`GameplayStatics.GetWorldDeltaSeconds`) _scale))
          (if (< _returnvalue_2 1.0)
            (`SceneComponent.SetWorldScale3D` (`self.SM_Body`) (`KismetMathLibrary.VLerp` (0.0 0.0 0.0) (1.0 1.0 1.0) _returnvalue_2))))))))

(event `UpdateDoors`
  (bind _sm_doora (`self.SM_DoorA`))
  (bind _sm_doorb (`self.SM_DoorB`))
  (bind _sm_doorc (`self.SM_DoorC`))
  (bind _sm_doorc_2 (`self.SM_DoorC`))
  (bind _sm_doora_2 (`self.SM_DoorA`))
  (bind _sm_doorb_2 (`self.SM_DoorB`))
  (`|ExecutionSequence`
    (:`then_0`
      (`ChildActorComponent.SetChildActorClass` (`self.BP_WeaponA`) (`self.WeaponA`))
      (`ChildActorComponent.SetChildActorClass` (`self.BP_WeaponB`) (`self.WeaponB`))
      (`ChildActorComponent.SetChildActorClass` (`self.BP_WeaponC`) (`self.WeaponC`)))
    (:`then_1`
      (if (`self.bIsOpen`)
        (`SceneComponent.K2_SetRelativeLocation` _sm_doora (`KismetMathLibrary.MakeVector` (.x (`SceneComponent.RelativeLocation` _sm_doora)) (.y (`SceneComponent.RelativeLocation` _sm_doora)) (`self.ZOffsetUp`)) false false)
        (`SceneComponent.K2_SetRelativeLocation` _sm_doorb (`KismetMathLibrary.MakeVector` (.x (`SceneComponent.RelativeLocation` _sm_doorb)) (.y (`SceneComponent.RelativeLocation` _sm_doorb)) (`self.ZOffsetUp`)) false false)
        (`SceneComponent.K2_SetRelativeLocation` _sm_doorc (`KismetMathLibrary.MakeVector` (.x (`SceneComponent.RelativeLocation` _sm_doorc)) (.y (`SceneComponent.RelativeLocation` _sm_doorc)) (`self.ZOffsetUp`)) false false)
        (else
          (`SceneComponent.K2_SetRelativeLocation` _sm_doora_2 (`KismetMathLibrary.MakeVector` (.x (`SceneComponent.RelativeLocation` _sm_doora_2)) (.y (`SceneComponent.RelativeLocation` _sm_doora_2)) (`self.ZOffsetDown`)) false false)
          (`SceneComponent.K2_SetRelativeLocation` _sm_doorb_2 (`KismetMathLibrary.MakeVector` (.x (`SceneComponent.RelativeLocation` _sm_doorb_2)) (.y (`SceneComponent.RelativeLocation` _sm_doorb_2)) (`self.ZOffsetDown`)) false false)
          (`SceneComponent.K2_SetRelativeLocation` _sm_doorc_2 (`KismetMathLibrary.MakeVector` (.x (`SceneComponent.RelativeLocation` _sm_doorc_2)) (.y (`SceneComponent.RelativeLocation` _sm_doorc_2)) (`self.ZOffsetDown`)) false false))))))

(fn `UserConstructionScript`
  (`self.UpdateDoors`))