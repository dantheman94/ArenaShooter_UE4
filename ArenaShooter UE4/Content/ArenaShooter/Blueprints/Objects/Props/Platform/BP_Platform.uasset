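; BP_Platform is an arena prop that rises along a spline after a configurable delay into the match.
; It starts at the spline's last point, and a timeline serves as a tick to move it toward point zero.
; Each update subtracts a curve-driven speed, sampled by straight-line distance to the top, from its spline distance until it arrives.
; The construction script places arrows marking both ends of the path.
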(event `self.ReceiveBeginPlay`
  (bind _spl_risingpath (`self.SPL_RisingPath`))
  (`SceneComponent.K2_SetWorldLocation` (`self.PlatformRootChild`) (`SplineComponent.GetLocationAtSplinePoint` _spl_risingpath (`SplineComponent.GetNumberOfSplinePoints` _spl_risingpath) "World") false false)
  (`KismetSystemLibrary.Delay` (`self.InitiateSecondsIntoTheMatch`))
  (`self.StartRisingProcedure`))

(event `StartRisingProcedure`
  (bind _spl_risingpath (`self.SPL_RisingPath`))
  (bind _returnvalue (`SplineComponent.GetLocationAtSplinePoint` _spl_risingpath 0 "World"))
  (`SceneComponent.K2_SetWorldLocation` (`self.PlatformRootChild`) (`SplineComponent.GetLocationAtSplinePoint` _spl_risingpath (`SplineComponent.GetNumberOfSplinePoints` _spl_risingpath) "World") false false)
  (set `self.DistanceAlongSpline` (`KismetMathLibrary.Vector_Distance` (`SceneComponent.K2_GetComponentLocation` (`self.SM_Body`)) _returnvalue))
  (`Timeline|TimelineUpdate` :!label _label
    (:`Update`
      (bind _output_get (set `self.DistanceAlongSpline` (- (`self.DistanceAlongSpline`) (* (`GameplayStatics.GetWorldDeltaSeconds`) (`CurveFloat.GetFloatValue` (`self.LandingSpeed`) (`KismetMathLibrary.Vector_Distance` (`SceneComponent.K2_GetComponentLocation` (`self.SM_Body`)) _returnvalue))))))
      (if (>= _output_get -5.0)
        (`SceneComponent.K2_SetWorldLocation` (`self.PlatformRootChild`) (`SplineComponent.GetLocationAtDistanceAlongSpline` (`self.SPL_RisingPath`) (`self.DistanceAlongSpline`) "World") false false)
        (else
          (`|ExecutionSequence`
            (:`then_0`
              (`/Engine/EditorBlueprintResources/StandardMacros.DoOnce` false))
            (:`then_1`
              (goto _label :!via `Stop`))))))))

(fn `UserConstructionScript`
  (bind _spl_risingpath (`self.SPL_RisingPath`))
  (`SceneComponent.K2_SetWorldLocation` (`self.ArrowBottom`) (`SplineComponent.GetLocationAtSplinePoint` _spl_risingpath (`SplineComponent.GetNumberOfSplinePoints` _spl_risingpath) "World") false false)
  (`SceneComponent.K2_SetWorldLocation` (`self.ArrowTop`) (+ (`SplineComponent.GetLocationAtSplinePoint` _spl_risingpath 0 "World") (0.0 0.0 100.0)) false false))