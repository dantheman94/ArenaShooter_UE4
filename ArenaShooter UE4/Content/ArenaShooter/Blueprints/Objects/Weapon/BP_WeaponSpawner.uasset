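; Arena weapon spawner that places the weapon configured in WeaponToSpawn at its skeletal mesh's transform.
; The construction script previews the weapon's mesh, which BeginPlay clears before spawning immediately or after FRespawnTime, depending on SpawnAtStart.
; RPC-named events handle spawning and the delay, then bind the spawned interactable's OnInteraction to an empty handler.
; The pickup-to-respawn timer binding is disconnected, so pickups trigger no respawn here.
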(event `self.ReceiveBeginPlay`
  (`SkinnedMeshComponent.SetSkinnedAssetAndUpdate` (`self.SkeletalMesh`) null true)
  (if (`self.bSpawnAtStart`)
    (`self.RPC_SpawnWeapon`)
    (else
      (`self.RPC_StartTimer`))))

(event `RPC_SpawnWeapon`
  (bind _returnvalue (`|SpawnActorFromClass` (defaults `Object` (`self.WeaponToSpawn`)) (`SceneComponent.K2_GetComponentToWorld` (`self.SkeletalMesh`)) "AlwaysSpawn" "OverrideRootScale" null null))
  (bind _output_get (set `self.InteractableInstance` _returnvalue))
  (bind _asbp_interactable (cast `/Game/ArenaShooter/Blueprints/Objects/Attributes/Interaction/BP_Interactable` _output_get))
  (add `/Game/ArenaShooter/Blueprints/Objects/Attributes/Interaction/BP_Interactable.OnInteraction` _asbp_interactable (delegate `OnInteraction`)))

(event `OnInteraction`
  (params (Interactable :type "/Game/ArenaShooter/Blueprints/Objects/Attributes/Interaction/BP_Interactable Object Reference")))

(event `RPC_StartTimer`
  (`KismetSystemLibrary.Delay` (`self.fRespawnTime`))
  (`self.RPC_SpawnWeapon`))

(fn `UserConstructionScript`
  (`SkinnedMeshComponent.SetSkinnedAssetAndUpdate` (`self.SkeletalMesh`) (defaults `Object` (`self.WeaponToSpawn`)) true))