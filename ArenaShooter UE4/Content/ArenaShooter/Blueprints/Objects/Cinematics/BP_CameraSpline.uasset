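; BP_CameraSpline is a cinematic helper actor that visualizes a camera spline around a focal point at the actor's origin.
; Its construction script labels a text render with the actor's display name plus "Focal Point".
; It then adds an arrow component at each spline point and rotates it to look at the actor's location, previewing view direction.
; It has no runtime logic of its own.
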(fn `UserConstructionScript`
  (bind __spline (`self._Spline`))
  (`parent.UserConstructionScript`)
  (`TextRenderComponent.K2_SetText` (`self.TextRender`) (`KismetTextLibrary.Conv_StringToText` (`KismetStringLibrary.Concat_StrStr` (`KismetSystemLibrary.GetDisplayName` self) " \nFocal Point")))
  (for _index (range (`SplineComponent.GetNumberOfSplinePoints` __spline))
    (bind _returnvalue (`AddComponent|NODE_AddArrowComponent-0` :`RelativeTransform` (`SplineComponent.GetTransformAtSplinePoint` __spline _index "Local" false)))
    (`SceneComponent.K2_SetWorldRotation` _returnvalue (`KismetMathLibrary.FindLookAtRotation` (`SceneComponent.K2_GetComponentLocation` _returnvalue) (`self.K2_GetActorLocation`)) false false)))