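; Editor helper Blueprint that, judging by its name, is used to author first-person weapon origin transforms for the submachine gun's aiming pose.
; The construction script hides the Mesh and both dual-wield arm meshes along with their children.
; Disconnected logic holds a dual-wield setup that hides weapon meshes and left upper-arm bones, plus creation of a SightPoint sphere at the primary weapon's AimingCameraPoint socket.
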(fn `UserConstructionScript`
  (`SceneComponent.SetVisibility` (`self.Mesh`) false true)
  (`SceneComponent.SetVisibility` (`self._FirstPerson_ArmsDuelRight`) false true)
  (`SceneComponent.SetVisibility` (`self._FirstPerson_ArmsDuelLeft`) false true))