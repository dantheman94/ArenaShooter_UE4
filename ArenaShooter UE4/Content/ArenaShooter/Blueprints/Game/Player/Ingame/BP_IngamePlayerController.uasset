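; In-game player controller that toggles the pause screen from the PauseGameplay input or its Unpause event.
; A shared FlipFlop alternates between showing the cursor and W_PauseScreen with HUD hidden and input disabled, and reversing that state.
; The pause widget is created on first use and reused.
; Game time is not paused here; only the controller's input is disabled.
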(event `Unpause`
  (bind _w_pausescreen (`self.w_PauseScreen`))
  (if (stale _isa)
    (bind _isa (`/Engine/EditorBlueprintResources/StandardMacros.FlipFlop` :!label _label)
      (:`A`
        (set `self.bShowMouseCursor` true)
        (`self.DisableInput` self)
        (bind _asbp_ingame_hud (cast `/Game/ArenaShooter/Blueprints/Game/Player/Ingame/BP_IngameHUD` (`self.GetHUD`)))
        (`BaseHUD.SetDisplayHud` _asbp_ingame_hud false)
        (`/Engine/EditorBlueprintResources/StandardMacros.IsValid` (`self.w_PauseScreen`)
          (:`Is Valid`
            _)
          (:`Is Not Valid`
            (bind _returnvalue (`|CreateWidget` "/Game/ArenaShooter/UMG/Ingame/Screens/w_PauseScreen.w_PauseScreen_C" self))
            (bind _output_get (set `self.w_PauseScreen` _returnvalue))))
        (if (not (`Widget.IsInViewport` _output_get))
          (`UserWidget.AddToViewport` (`self.w_PauseScreen`) 0)))
      (:`B`
        (set `self.bShowMouseCursor` false)
        (`self.EnableInput` self)
        (bind _asbp_ingame_hud_2 (cast `/Game/ArenaShooter/Blueprints/Game/Player/Ingame/BP_IngameHUD` (`self.GetHUD`)))
        (`BaseHUD.SetDisplayHud` _asbp_ingame_hud_2 true)
        (`/Engine/EditorBlueprintResources/StandardMacros.IsValid` _w_pausescreen
          (:`Is Valid`
            (if (`Widget.IsInViewport` _w_pausescreen)
              (`Widget.RemoveFromParent` _w_pausescreen))))))))

(event `InputAction|PauseGameplay`
  (params (Key :type "Key Structure"))
  (:`Pressed`
    (if true
      (goto _label))))

(fn `UserConstructionScript`
  (`parent.UserConstructionScript`))