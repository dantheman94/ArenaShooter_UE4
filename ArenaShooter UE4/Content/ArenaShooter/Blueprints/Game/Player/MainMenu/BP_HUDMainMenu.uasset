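; Main menu HUD Blueprint that shows and hides the front-end UI: splash, menus, matchmaking, server browser, custom-game lists, lobbies, roster and loading screen.
; Each Show event calls its parent, lazily creates and caches the widget from a class variable, adds it to the viewport, and usually takes a Z-order.
; Lobby events choose host or client screens from a Hosting flag.
; Showing the roster also refreshes the game state's player list.
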(event `HideAllMainMenus`
  (bind __ui_lobbyroster_instance (`self._UI_LobbyRoster_Instance`))
  (bind __ui_mainmenu_instance (`self._UI_MainMenu_Instance`))
  (bind __ui_hostlobby_instance (`self._UI_HostLobby_Instance`))
  (bind __ui_clientlobby_instance (`self._UI_ClientLobby_Instance`))
  (`|ExecutionSequence`
    (:`then_0`
      (`/Engine/EditorBlueprintResources/StandardMacros.IsValid` __ui_mainmenu_instance
        (:`Is Valid`
          (`Widget.RemoveFromParent` __ui_mainmenu_instance))))
    (:`then_1`
      (`/Engine/EditorBlueprintResources/StandardMacros.IsValid` __ui_hostlobby_instance
        (:`Is Valid`
          (`Widget.RemoveFromParent` __ui_hostlobby_instance))))
    (:`then_2`
      (`/Engine/EditorBlueprintResources/StandardMacros.IsValid` __ui_clientlobby_instance
        (:`Is Valid`
          (`Widget.RemoveFromParent` __ui_clientlobby_instance))))
    (:`then_3`
      (`/Engine/EditorBlueprintResources/StandardMacros.IsValid` __ui_lobbyroster_instance
        (:`Is Valid`
          (`Widget.RemoveFromParent` __ui_lobbyroster_instance))))))

(event `self.ShowUI_LobbyMainMenu`
  (params (Hosting :type Boolean) (ZOrder :type Integer))
  (`parent.ShowUI_LobbyMainMenu` Hosting ZOrder)
  (`self.HideUI_MainMenu`)
  (`self.HideUI_ClientLobby`)
  (if Hosting
    (`self.ShowUI_MainMenu` ZOrder)
    (else
      (`self.ShowUI_ClientLobby` ZOrder))))

(event `self.ShowUI_Splash`
  ;[0 0 0] Local Main Pages
  ; - Splash
  ; - Main Menu
  ; - Matchmaking
  (`parent.ShowUI_Splash`)
  (`/Engine/EditorBlueprintResources/StandardMacros.IsValid` (`self._UI_SplashScreen_Instance`)
    (:`Is Valid`
      (if (not (`Widget.IsInViewport` (stale _output_get))) :!label _label
        (`UserWidget.AddToViewport` (`self._UI_SplashScreen_Instance`) 0)))
    (:`Is Not Valid`
      (if (`KismetSystemLibrary.IsValidClass` (`self._UI_SplashScreen_Class`))
        (bind _returnvalue (`|CreateWidget` (`self._UI_SplashScreen_Class`) (`self.GetOwningPlayerController`)))
        (bind _output_get (set `self._UI_SplashScreen_Instance` _returnvalue))
        (goto _label)
        (else
          (`KismetSystemLibrary.PrintString` (`KismetStringLibrary.Concat_StrStr` "ERROR: {" "_UI_SplashScreen_Class" "} is NULL in: " (`KismetSystemLibrary.GetClassDisplayName` (`GameplayStatics.GetObjectClass` self))) true false (struct :`R` 1.0 :`A` 1.0) 5.0))))))

(event `self.ShowUI_Playlist`
  (params (ZOrder :type Integer))
  (bind __ui_playlist_class (`self._UI_Playlist_Class`))
  ;[0 0 0] Local Sub Pages
  ; - Playlists
  ; - Server Browser
  ; - Map List (Custom Games)
  ; - Gamemode List (Custom Games)
  (`parent.ShowUI_Playlist` ZOrder)
  (`/Engine/EditorBlueprintResources/StandardMacros.IsValid` (`self._UI_Playlist_Instance`)
    (:`Is Valid`
      (if (not (`Widget.IsInViewport` (stale _output_get))) :!label _label_2
        (`UserWidget.AddToViewport` (`self._UI_Playlist_Instance`) ZOrder)))
    (:`Is Not Valid`
      (if (`KismetSystemLibrary.IsValidClass` __ui_playlist_class)
        (bind _returnvalue (`|CreateWidget` __ui_playlist_class (`self.GetOwningPlayerController`)))
        (bind _output_get (set `self._UI_Playlist_Instance` _returnvalue))
        (goto _label_2)
        (else
          (`KismetSystemLibrary.PrintString` (`KismetStringLibrary.Concat_StrStr` "ERROR: {" "_UI_Playlist_Class" "} is NULL in: " (`KismetSystemLibrary.GetClassDisplayName` (`GameplayStatics.GetObjectClass` self))) true false (struct :`R` 1.0 :`A` 1.0) 5.0))))))

(event `self.ShowUI_SearchingForGames`
  (params (ZOrder :type Integer))
  (bind __ui_searchingformatch_class (`self._UI_SearchingForMatch_Class`))
  ;[0 0 0] Lobby Main Pages
  ; - Custom Games
  ; - Searching For Games
  ; - Pre Match Lobby Screen,
  ; - Non-Host Screen
  (`parent.ShowUI_SearchingForGames` ZOrder)
  (`/Engine/EditorBlueprintResources/StandardMacros.IsValid` (`self._UI_SearchingForMatch_Instance`)
    (:`Is Valid`
      (if (not (`Widget.IsInViewport` (stale _output_get))) :!label _label_3
        (`UserWidget.AddToViewport` (`self._UI_SearchingForMatch_Instance`) ZOrder)))
    (:`Is Not Valid`
      (if (`KismetSystemLibrary.IsValidClass` __ui_searchingformatch_class)
        (bind _returnvalue (`|CreateWidget` __ui_searchingformatch_class (`self.GetOwningPlayerController`)))
        (bind _output_get (set `self._UI_SearchingForMatch_Instance` _returnvalue))
        (goto _label_3)
        (else
          (`KismetSystemLibrary.PrintString` (`KismetStringLibrary.Concat_StrStr` "ERROR: {" "_UI_SearchingForMatch_Class" "} is NULL in: " (`KismetSystemLibrary.GetClassDisplayName` (`GameplayStatics.GetObjectClass` self))) true false (struct :`R` 1.0 :`A` 1.0) 5.0))))))

(event `self.ShowUI_LobbyRoster`
  (params (ZOrder :type Integer))
  (bind __ui_lobbyroster_instance (`self._UI_LobbyRoster_Instance`))
  ;[0 0 0] Lobby Overlays
  ; - Roster
  ; - Loading Screen
  (`parent.ShowUI_LobbyRoster` ZOrder)
  (`/Engine/EditorBlueprintResources/StandardMacros.IsValid` __ui_lobbyroster_instance
    (:`Is Valid`
      (`Widget.RemoveFromParent` __ui_lobbyroster_instance)
      (if (not (`Widget.IsInViewport` (stale _output_get))) :!label _label_4
        (`UserWidget.AddToViewport` (`self._UI_LobbyRoster_Instance`) ZOrder)
        (bind _asbase_game_state (cast `BaseGameState` (`GameplayStatics.GetGameState`)))
        (`BaseGameState.UpdatePlayerList` _asbase_game_state)
        (bind _asw_roster (cast `/Game/ArenaShooter/UMG/MainMenu/Lobby/Overlays/w_Roster` (stale _output_get)))
        (`Widget.SetVisibility` (`/Game/ArenaShooter/UMG/MainMenu/Lobby/Overlays/w_Roster.PlayerLists` _asw_roster) "Visible")))
    (:`Is Not Valid`
      (if (`KismetSystemLibrary.IsValidClass` (`self._UI_LobbyRoster_Class`))
        (bind _returnvalue (`|CreateWidget` (`self._UI_LobbyRoster_Class`) (`self.GetOwningPlayerController`)))
        (bind _output_get (set `self._UI_LobbyRoster_Instance` _returnvalue))
        (goto _label_4)
        (else
          (`KismetSystemLibrary.PrintString` (`KismetStringLibrary.Concat_StrStr` "ERROR: {" "_UI_LobbyRoster_Class" "} is NULL in: " (`KismetSystemLibrary.GetClassDisplayName` (`GameplayStatics.GetObjectClass` self))) true false (struct :`R` 1.0 :`A` 1.0) 5.0))))))

(event `self.HideUI_LobbyRoster`
  (params (bHideListOnly :type Boolean))
  (bind __ui_lobbyroster_instance (`self._UI_LobbyRoster_Instance`))
  ;[0 0 0] Lobby Overlays
  ; - Roster
  ; - Loading Screen
  (if bHideListOnly
    (`/Engine/EditorBlueprintResources/StandardMacros.IsValid` __ui_lobbyroster_instance
      (:`Is Valid`
        (bind _asw_roster (cast `/Game/ArenaShooter/UMG/MainMenu/Lobby/Overlays/w_Roster` __ui_lobbyroster_instance))
        (`Widget.SetVisibility` (`/Game/ArenaShooter/UMG/MainMenu/Lobby/Overlays/w_Roster.PlayerLists` _asw_roster) "Hidden")))))

(event `self.ShowUI_LobbyPrematch`
  (params (Hosting :type Boolean) (ZOrder :type Integer))
  (`parent.ShowUI_LobbyPrematch` Hosting ZOrder)
  (`self.HideUI_HostLobby`)
  (`self.HideUI_ClientLobby`)
  (if Hosting
    (`self.ShowUI_HostLobby` ZOrder)
    (else
      (`self.ShowUI_ClientLobby` ZOrder))))

(event `self.ShowUI_MainMenu`
  (params (ZOrder :type Integer))
  ;[0 0 0] Local Main Pages
  ; - Splash
  ; - Main Menu
  ; - Matchmaking
  (`parent.ShowUI_MainMenu` ZOrder)
  (`/Engine/EditorBlueprintResources/StandardMacros.IsValid` (`self._UI_MainMenu_Instance`)
    (:`Is Valid`
      (if (not (`Widget.IsInViewport` (stale _output_get))) :!label _label_5
        (`UserWidget.AddToViewport` (`self._UI_MainMenu_Instance`) ZOrder)))
    (:`Is Not Valid`
      (if (`KismetSystemLibrary.IsValidClass` (`self._UI_MainMenu_Class`))
        (bind _returnvalue (`|CreateWidget` (`self._UI_MainMenu_Class`) (`self.GetOwningPlayerController`)))
        (bind _output_get (set `self._UI_MainMenu_Instance` _returnvalue))
        (goto _label_5)
        (else
          (`KismetSystemLibrary.PrintString` (`KismetStringLibrary.Concat_StrStr` "ERROR: {" "_UI_MainMenu_Class" "} is NULL in: " (`KismetSystemLibrary.GetClassDisplayName` (`GameplayStatics.GetObjectClass` self))) true false (struct :`R` 1.0 :`A` 1.0) 5.0))))))

(event `self.ShowUI_ServerBrowser`
  (params (ZOrder :type Integer))
  (bind __ui_serverbrowser_class (`self._UI_ServerBrowser_Class`))
  ;[0 0 0] Local Sub Pages
  ; - Playlists
  ; - Server Browser
  ; - Map List (Custom Games)
  ; - Gamemode List (Custom Games)
  (`parent.ShowUI_ServerBrowser` ZOrder)
  (`/Engine/EditorBlueprintResources/StandardMacros.IsValid` (`self._UI_ServerBrowser_Instance`)
    (:`Is Valid`
      (if (not (`Widget.IsInViewport` (stale _output_get))) :!label _label_6
        (`UserWidget.AddToViewport` (`self._UI_ServerBrowser_Instance`) ZOrder)))
    (:`Is Not Valid`
      (if (`KismetSystemLibrary.IsValidClass` __ui_serverbrowser_class)
        (bind _returnvalue (`|CreateWidget` __ui_serverbrowser_class (`self.GetOwningPlayerController`)))
        (bind _output_get (set `self._UI_ServerBrowser_Instance` _returnvalue))
        (goto _label_6)
        (else
          (`KismetSystemLibrary.PrintString` (`KismetStringLibrary.Concat_StrStr` "ERROR: {" "_UI_ServerBrowser_Class" "} is NULL in: " (`KismetSystemLibrary.GetClassDisplayName` (`GameplayStatics.GetObjectClass` self))) true false (struct :`R` 1.0 :`A` 1.0) 5.0))))))

(event `self.ShowUI_LoadingServer`
  (params (Message :type "Text (by ref)") (ZOrder :type Integer))
  (bind __ui_loadingserver_instance (`self._UI_LoadingServer_Instance`))
  ;[0 0 0] Lobby Overlays
  ; - Roster
  ; - Loading Screen
  (`parent.ShowUI_LoadingServer` Message ZOrder)
  (`/Engine/EditorBlueprintResources/StandardMacros.IsValid` (`self._UI_LoadingServer_Instance`)
    (:`Is Valid`
      (if (not (`Widget.IsInViewport` (stale _output_get))) :!label _label_7
        (`UserWidget.AddToViewport` __ui_loadingserver_instance ZOrder)
        (bind _asw_loading_screen (cast `/Game/ArenaShooter/UMG/MainMenu/Local/w_LoadingScreen` __ui_loadingserver_instance))
        (set `/Game/ArenaShooter/UMG/MainMenu/Local/w_LoadingScreen.Text` Message _asw_loading_screen)))
    (:`Is Not Valid`
      (if (`KismetSystemLibrary.IsValidClass` (`self._UI_LoadingServer_Class`))
        (bind _returnvalue (`|CreateWidget` (`self._UI_LoadingServer_Class`) (`self.GetOwningPlayerController`)))
        (bind _output_get (set `self._UI_LoadingServer_Instance` _returnvalue))
        (goto _label_7)
        (else
          (`KismetSystemLibrary.PrintString` (`KismetStringLibrary.Concat_StrStr` "ERROR: {" "_UI_LoadingServer_Class" "} is NULL in: " (`KismetSystemLibrary.GetClassDisplayName` (`GameplayStatics.GetObjectClass` self))) true false (struct :`R` 1.0 :`A` 1.0) 5.0))))))

(event `self.ShowUI_BarracksHome`
  (params (ZOrder :type Integer))
  (bind __ui_barrackshome_class (`self._UI_BarracksHome_Class`))
  (`parent.ShowUI_BarracksHome` ZOrder)
  (`/Engine/EditorBlueprintResources/StandardMacros.IsValid` (`self._UI_BarracksHome_Instance`)
    (:`Is Valid`
      (if (not (`Widget.IsInViewport` (stale _output_get))) :!label _label_8
        (`UserWidget.AddToViewport` (`self._UI_BarracksHome_Instance`) ZOrder)))
    (:`Is Not Valid`
      (if (`KismetSystemLibrary.IsValidClass` __ui_barrackshome_class)
        (bind _returnvalue (`|CreateWidget` __ui_barrackshome_class (`self.GetOwningPlayerController`)))
        (bind _output_get (set `self._UI_BarracksHome_Instance` _returnvalue))
        (goto _label_8)
        (else
          (`KismetSystemLibrary.PrintString` (`KismetStringLibrary.Concat_StrStr` "ERROR: {" "_UI_BarracksHome_Class" "} is NULL in: " (`KismetSystemLibrary.GetClassDisplayName` (`GameplayStatics.GetObjectClass` self))) true false (struct :`R` 1.0 :`A` 1.0) 5.0))))))

(event `self.ShowUI_HostLobby`
  (params (ZOrder :type Integer))
  (bind __ui_hostlobby_instance (`self._UI_HostLobby_Instance`))
  (`parent.ShowUI_HostLobby` ZOrder)
  (`/Engine/EditorBlueprintResources/StandardMacros.IsValid` __ui_hostlobby_instance
    (:`Is Valid`
      (`Widget.RemoveFromParent` __ui_hostlobby_instance)
      (if (not (`Widget.IsInViewport` (stale _output_get))) :!label _label_9
        (`UserWidget.AddToViewport` (`self._UI_HostLobby_Instance`) ZOrder)))
    (:`Is Not Valid`
      (if (`KismetSystemLibrary.IsValidClass` (`self._UI_HostLobby_Class`))
        (bind _returnvalue (`|CreateWidget` (`self._UI_HostLobby_Class`) (`self.GetOwningPlayerController`)))
        (bind _output_get (set `self._UI_HostLobby_Instance` _returnvalue))
        (goto _label_9)
        (else
          (`KismetSystemLibrary.PrintString` "ERROR: _UI_HostLobby_Class is NULL" true false (struct :`R` 1.0 :`A` 1.0) 5.0))))))

(event `self.ShowUI_Matchmaking`
  (params (ZOrder :type Integer))
  (bind __ui_matchmaking_class (`self._UI_Matchmaking_Class`))
  ;[0 0 0] Local Main Pages
  ; - Splash
  ; - Main Menu
  ; - Matchmaking
  (`parent.ShowUI_Matchmaking` ZOrder)
  (`/Engine/EditorBlueprintResources/StandardMacros.IsValid` (`self._UI_Matchmaking_Instance`)
    (:`Is Valid`
      (if (not (`Widget.IsInViewport` (stale _output_get))) :!label _label_10
        (`UserWidget.AddToViewport` (`self._UI_Matchmaking_Instance`) ZOrder)))
    (:`Is Not Valid`
      (if (`KismetSystemLibrary.IsValidClass` __ui_matchmaking_class)
        (bind _returnvalue (`|CreateWidget` __ui_matchmaking_class (`self.GetOwningPlayerController`)))
        (bind _output_get (set `self._UI_Matchmaking_Instance` _returnvalue))
        (goto _label_10)
        (else
          (`KismetSystemLibrary.PrintString` (`KismetStringLibrary.Concat_StrStr` "ERROR: {" "_UI_Matchmaking_Class" "} is NULL in: " (`KismetSystemLibrary.GetClassDisplayName` (`GameplayStatics.GetObjectClass` self))) true false (struct :`R` 1.0 :`A` 1.0) 5.0))))))

(event `self.ShowUI_GameModeList`
  (params (ZOrder :type Integer))
  (bind __ui_gamemodelist_class (`self._UI_GameModeList_Class`))
  ;[0 0 0] Local Sub Pages
  ; - Playlists
  ; - Server Browser
  ; - Map List (Custom Games)
  ; - Gamemode List (Custom Games)
  (`parent.ShowUI_GameModeList` ZOrder)
  (`/Engine/EditorBlueprintResources/StandardMacros.IsValid` (`self._UI_GameModeList_Instance`)
    (:`Is Valid`
      (if (not (`Widget.IsInViewport` (stale _output_get))) :!label _label_11
        (`UserWidget.AddToViewport` (`self._UI_GameModeList_Instance`) ZOrder)))
    (:`Is Not Valid`
      (if (`KismetSystemLibrary.IsValidClass` __ui_gamemodelist_class)
        (bind _returnvalue (`|CreateWidget` __ui_gamemodelist_class (`self.GetOwningPlayerController`)))
        (bind _output_get (set `self._UI_GameModeList_Instance` _returnvalue))
        (goto _label_11)
        (else
          (`KismetSystemLibrary.PrintString` (`KismetStringLibrary.Concat_StrStr` "ERROR: {" "_UI_GameModeList_Class" "} is NULL in: " (`KismetSystemLibrary.GetClassDisplayName` (`GameplayStatics.GetObjectClass` self))) true false (struct :`R` 1.0 :`A` 1.0) 5.0))))))

(event `self.HideUI_HostLobby`
  (bind __ui_hostlobby_instance (`self._UI_HostLobby_Instance`))
  (`parent.HideUI_HostLobby`)
  (`/Engine/EditorBlueprintResources/StandardMacros.IsValid` __ui_hostlobby_instance
    (:`Is Valid`
      (`Widget.RemoveFromParent` __ui_hostlobby_instance))))

(event `self.ShowUI_SettingsHome`
  (params (ZOrder :type Integer))
  (bind __ui_settingshome_class (`self._UI_SettingsHome_Class`))
  (`parent.ShowUI_SettingsHome` ZOrder)
  (`/Engine/EditorBlueprintResources/StandardMacros.IsValid` (`self._UI_SettingsHome_Instance`)
    (:`Is Valid`
      (if (not (`Widget.IsInViewport` (stale _output_get))) :!label _label_12
        (`UserWidget.AddToViewport` (`self._UI_SettingsHome_Instance`) ZOrder)))
    (:`Is Not Valid`
      (if (`KismetSystemLibrary.IsValidClass` __ui_settingshome_class)
        (bind _returnvalue (`|CreateWidget` __ui_settingshome_class (`self.GetOwningPlayerController`)))
        (bind _output_get (set `self._UI_SettingsHome_Instance` _returnvalue))
        (goto _label_12)
        (else
          (`KismetSystemLibrary.PrintString` (`KismetStringLibrary.Concat_StrStr` "ERROR: {" "_UI_SettingsHome_Class" "} is NULL in: " (`KismetSystemLibrary.GetClassDisplayName` (`GameplayStatics.GetObjectClass` self))) true false (struct :`R` 1.0 :`A` 1.0) 5.0))))))

(event `self.ShowUI_ClientLobby`
  (params (ZOrder :type Integer))
  (bind __ui_clientlobby_instance (`self._UI_ClientLobby_Instance`))
  (`parent.ShowUI_ClientLobby` ZOrder)
  (`/Engine/EditorBlueprintResources/StandardMacros.IsValid` __ui_clientlobby_instance
    (:`Is Valid`
      (`Widget.RemoveFromParent` __ui_clientlobby_instance)
      (if (not (`Widget.IsInViewport` (stale _output_get))) :!label _label_13
        (`UserWidget.AddToViewport` (`self._UI_ClientLobby_Instance`) ZOrder)))
    (:`Is Not Valid`
      (if (`KismetSystemLibrary.IsValidClass` (`self._UI_ClientLobby_Class`))
        (bind _returnvalue (`|CreateWidget` (`self._UI_ClientLobby_Class`) (`self.GetOwningPlayerController`)))
        (bind _output_get (set `self._UI_ClientLobby_Instance` _returnvalue))
        (goto _label_13)
        (else
          (`KismetSystemLibrary.PrintString` "ERROR: _UI_ClientLobby_Class is NULL" true false (struct :`R` 1.0 :`A` 1.0) 5.0))))))

(event `self.ShowUI_MapList`
  (params (ZOrder :type Integer))
  (bind __ui_maplist_class (`self._UI_MapList_Class`))
  ;[0 0 0] Local Sub Pages
  ; - Playlists
  ; - Server Browser
  ; - Map List (Custom Games)
  ; - Gamemode List (Custom Games)
  (`parent.ShowUI_MapList` ZOrder)
  (`/Engine/EditorBlueprintResources/StandardMacros.IsValid` (`self._UI_MapList_Instance`)
    (:`Is Valid`
      (if (not (`Widget.IsInViewport` (stale _output_get))) :!label _label_14
        (`UserWidget.AddToViewport` (`self._UI_MapList_Instance`) ZOrder)))
    (:`Is Not Valid`
      (if (`KismetSystemLibrary.IsValidClass` __ui_maplist_class)
        (bind _returnvalue (`|CreateWidget` __ui_maplist_class (`self.GetOwningPlayerController`)))
        (bind _output_get (set `self._UI_MapList_Instance` _returnvalue))
        (goto _label_14)
        (else
          (`KismetSystemLibrary.PrintString` (`KismetStringLibrary.Concat_StrStr` "ERROR: {" "_UI_MapList_Class" "} is NULL in: " (`KismetSystemLibrary.GetClassDisplayName` (`GameplayStatics.GetObjectClass` self))) true false (struct :`R` 1.0 :`A` 1.0) 5.0))))))

(event `self.HideUI_ClientLobby`
  (bind __ui_clientlobby_instance (`self._UI_ClientLobby_Instance`))
  (`parent.HideUI_ClientLobby`)
  (`/Engine/EditorBlueprintResources/StandardMacros.IsValid` __ui_clientlobby_instance
    (:`Is Valid`
      (`Widget.RemoveFromParent` __ui_clientlobby_instance))))

(fn `UserConstructionScript`)