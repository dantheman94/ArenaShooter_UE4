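; In-game Game State Blueprint that runs the match intro, from opening cinematic to player control.
; With the cinematic enabled, it shows loading and title widgets, hides HUDs, then waits for the cinematic's head-zoom threshold.
; It then either opens the buy menu with input locked, or shows HUDs and signals intro completion after a delay.
; Intro completion restores game input and HUDs and adds a match title; fade-screen chains are disconnected.
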(event `self.ReceiveBeginPlay`
  (add `self.IntroSequenceComplete` (delegate `BindIntroSequenceComplete`))
  (if (`self._bPlayOpeningCinematic`)
    (bind _returnvalue (`|CreateWidget` "/Game/ArenaShooter/UMG/Ingame/Screens/w_LoadingPlayers.w_LoadingPlayers_C" (`GameplayStatics.GetPlayerController` 0)))
    (`UserWidget.AddToViewport` _returnvalue 0)
    (`|ExecutionSequence`
      (:`then_0`
        (`KismetSystemLibrary.Delay` (`/Game/ArenaShooter/UMG/Ingame/Screens/w_LoadingPlayers.Delay` _returnvalue))
        (bind _returnvalue_2 (`|CreateWidget` "/Game/ArenaShooter/UMG/Ingame/Screens/w_IngameMatchTitle.w_IngameMatchTitle_C" (`GameplayStatics.GetPlayerController` 0)))
        (bind _output_get (set `self.MatchTitle` _returnvalue_2))
        (`UserWidget.AddToViewport` _output_get 0)
        (for _array_element (`self.PlayerArray`)
          (bind _asbase_player_state (cast `BasePlayerState` _array_element))
          (bind ((`_PlayerController` __playercontroller)) (break `PlayerInfo` (`BasePlayerState._PlayerInfo` _asbase_player_state)))
          (`/Engine/EditorBlueprintResources/StandardMacros.IsValid` __playercontroller
            (:`Is Valid`
              (bind _asbp_ingame_hud (cast `/Game/ArenaShooter/Blueprints/Game/Player/Ingame/BP_IngameHUD` (`PlayerController.GetHUD` __playercontroller)))
              (`BaseHUD.SetDisplayHud` _asbp_ingame_hud false)))))
      (:`then_1`
        (for _array_element_2 (`self._tOpeningCinematics`)
          (`/Engine/EditorBlueprintResources/StandardMacros.IsValid` _array_element_2
            (:`Is Valid`
              (add `CameraCinematic._OnCinematicStart` _array_element_2 (delegate `OnCinematicStart`))
              (add `CameraCinematic._OnHeadZoomThreshold` _array_element_2 (delegate `OnHeadZoomThreshold`)))))))
    (else
      (`KismetSystemLibrary.Delay` 0.0)
      (`self.BuyMenuSequence`))))

(event `BindIntroSequenceComplete`
  (`self.IntroSequenceCompleteEvent`))

(event `OnCinematicStart`
  ;[0 0 0] Fade In
)

(event `OnHeadZoomThreshold`
  ;[0 0 0] Fade Out
  (`/Engine/EditorBlueprintResources/StandardMacros.DoOnce` false
    (:`Completed`
      (`KismetSystemLibrary.Delay` 0.15)
      (`self.BuyMenuSequence`))))

(event `BuyMenuSequence`
  (bind _localplayercontroller (`self.LocalPlayerController`))
  (bind _matchtitle (`self.MatchTitle`))
  (if (`self._bShowBuyMenu`)
    (bind _returnvalue (`|CreateWidget` "/Game/ArenaShooter/UMG/Ingame/Screens/BuyMenu/w_BuyMenu_V2.w_BuyMenu_V2_C" (`GameplayStatics.GetPlayerController` 0)))
    (`UserWidget.AddToViewport` _returnvalue 0)
    (for _array_element (`self.PlayerArray`)
      (bind _asbase_player_state (cast `BasePlayerState` _array_element))
      (bind ((`_PlayerController` __playercontroller)) (break `PlayerInfo` (`BasePlayerState._PlayerInfo` _asbase_player_state)))
      (`/Engine/EditorBlueprintResources/StandardMacros.IsValid` __playercontroller
        (:`Is Valid`
          (bind _output_get (set `self.LocalPlayerController` __playercontroller))
          (set `PlayerController.bShowMouseCursor` true _output_get)
          (`WidgetBlueprintLibrary.SetInputMode_UIOnlyEx` _output_get _returnvalue "LockAlways")
          (`Controller.SetIgnoreLookInput` _output_get true)
          (`Controller.SetIgnoreMoveInput` _output_get true)
          (`/Engine/EditorBlueprintResources/StandardMacros.IsValid` _matchtitle :!label _label
            (:`Is Valid`
              (`Widget.RemoveFromParent` _matchtitle))
            (:`Is Not Valid`
              _))
          (`PlayerController.SetViewTargetWithBlend` _localplayercontroller (`Controller.K2_GetPawn` _localplayercontroller) 0.0 "VTBlend_Linear" 0.0 false))))
    (else
      ;[0 0 0] Show Hud
      (for _array_element_2 (`self.PlayerArray`)
        (bind _asbase_player_state_2 (cast `BasePlayerState` _array_element_2))
        (bind ((`_PlayerController` __playercontroller_2)) (break `PlayerInfo` (`BasePlayerState._PlayerInfo` _asbase_player_state_2)))
        (`/Engine/EditorBlueprintResources/StandardMacros.IsValid` __playercontroller_2
          (:`Is Valid`
            (bind _output_get_2 (set `self.LocalPlayerController` __playercontroller_2))
            (bind _asbp_ingame_hud (cast `/Game/ArenaShooter/Blueprints/Game/Player/Ingame/BP_IngameHUD` (`PlayerController.GetHUD` _output_get_2)))
            (`BaseHUD.SetDisplayHud` _asbp_ingame_hud true)
            (`|ExecutionSequence`
              (:`then_0`
                (goto _label))
              (:`then_1`
                (`KismetSystemLibrary.Delay` 1.0)
                (`self.IntroSequenceComplete`)))))))))

(event `IntroSequenceCompleteEvent`
  (for _array_element (`self.PlayerArray`)
    (bind _asbase_player_state (cast `BasePlayerState` _array_element))
    (bind ((`_PlayerController` __playercontroller)) (break `PlayerInfo` (`BasePlayerState._PlayerInfo` _asbase_player_state)))
    (`/Engine/EditorBlueprintResources/StandardMacros.IsValid` __playercontroller
      (:`Is Valid`
        (bind _output_get (set `self.LocalPlayerController` __playercontroller))
        (set `PlayerController.bShowMouseCursor` false _output_get)
        (`WidgetBlueprintLibrary.SetInputMode_GameOnly` _output_get)
        (`Controller.SetIgnoreLookInput` _output_get false)
        (`Controller.SetIgnoreMoveInput` _output_get false)
        (bind _asbp_ingame_hud (cast `/Game/ArenaShooter/Blueprints/Game/Player/Ingame/BP_IngameHUD` (`PlayerController.GetHUD` __playercontroller)))
        (`BaseHUD.SetDisplayHud` _asbp_ingame_hud true))))
  (bind _returnvalue (`|CreateWidget` "/Game/ArenaShooter/UMG/Ingame/HUD/Multiplayer/w_MatchTitle.w_MatchTitle_C" (`GameplayStatics.GetPlayerController` 0)))
  (`UserWidget.AddToViewport` _returnvalue 0))

(fn `UserConstructionScript`)